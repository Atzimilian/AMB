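; Ambient sound Blueprint that plays one-shot environmental cues at random positions around the world origin.
; On BeginPlay it starts wind and falling-rock loops, each a function timer with a random delay that plays its sound and re-arms itself.
; Wind plays at random sky positions and rock sounds below ground level.
; Crow and vulture loops follow the same pattern but are never started.
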(event `self.ReceiveBeginPlay`
  (`self.CueAudio`))

(event `CueAudio`
  (`self.SetWindTimer`)
  (`self.SetStoneTimer`))

(event `SetCrowTimer`
  (bind _delay (`self.GetDelay` 5.0 20.0))
  (`KismetSystemLibrary.K2_SetTimer` null "PlayCrow" _delay))

(event `SetVultureTimer`
  (bind _delay (`self.GetDelay` 5.0 20.0))
  (`KismetSystemLibrary.K2_SetTimer` null "PlayVulture" _delay))

(event `SetWindTimer`
  (bind _delay (`self.GetDelay` 5.0 20.0))
  (`KismetSystemLibrary.K2_SetTimer` null "PlayWind" _delay))

(event `SetStoneTimer`
  (bind _delay (`self.GetDelay` 5.0 20.0))
  (`KismetSystemLibrary.K2_SetTimer` null "PlayStone" _delay))

(fn `GetDelay`
  (params (Min :type "Float (double-precision)") (Max :type "Float (double-precision)"))
  (returns (Delay :type "Float (double-precision)"))
  (return (`KismetMathLibrary.Lerp` Min Max (`KismetMathLibrary.RandomFloat`))))

(fn `GetRandomSkyLocation`
  (returns (SkyLocation :type "Vector Structure"))
  (return (`KismetMathLibrary.MakeVector` (`KismetMathLibrary.Lerp` 7500.0 -7500.0 (`KismetMathLibrary.RandomFloat`)) (`KismetMathLibrary.Lerp` 7500.0 -7500.0 (`KismetMathLibrary.RandomFloat`)) (`KismetMathLibrary.Lerp` 400.0 2000.0 (`KismetMathLibrary.RandomFloat`)))))

(fn `GetRandomStoneLocation`
  (returns (SkyLocation :type "Vector Structure"))
  (return (`KismetMathLibrary.MakeVector` (`KismetMathLibrary.Lerp` 7500.0 -7500.0 (`KismetMathLibrary.RandomFloat`)) (`KismetMathLibrary.Lerp` 7500.0 -7500.0 (`KismetMathLibrary.RandomFloat`)) (`KismetMathLibrary.Lerp` 0.0 -1000.0 (`KismetMathLibrary.RandomFloat`)))))

(fn `PlayCrow`
  (bind _skylocation (`self.GetRandomSkyLocation`))
  (`GameplayStatics.PlaySoundAtLocation` "/Game/07_Audio/03_SFX_Ambient/Krähe_Pixabay_pixabay_Cue.Krähe_Pixabay_pixabay_Cue" _skylocation (struct) 1.0 1.0 0.0 null null null null)
  (`self.SetCrowTimer`))

(fn `PlayStone`
  (bind _skylocation (`self.GetRandomStoneLocation`))
  (`GameplayStatics.PlaySoundAtLocation` "/Game/07_Audio/03_SFX_Ambient/BrechendeFelsen_Freesound_org_AGC66_Cue.BrechendeFelsen_Freesound_org_AGC66_Cue" _skylocation (struct) 1.0 1.0 0.0 null null null null)
  (`self.SetStoneTimer`))

(fn `PlayVulture`
  (bind _skylocation (`self.GetRandomSkyLocation`))
  (`GameplayStatics.PlaySoundAtLocation` "/Game/07_Audio/03_SFX_Ambient/Geier_Pixabay_pixabay_Cue.Geier_Pixabay_pixabay_Cue" _skylocation (struct) 1.0 1.0 0.0 null null null null)
  (`self.SetVultureTimer`))

(fn `PlayWind`
  (bind _skylocation (`self.GetRandomSkyLocation`))
  (`GameplayStatics.PlaySoundAtLocation` "/Game/07_Audio/03_SFX_Ambient/WindLow_Freesoound_org_chiu29_Cue.WindLow_Freesoound_org_chiu29_Cue" _skylocation (struct) 1.0 1.0 0.0 null null null null)
  (`self.SetWindTimer`))

(fn `UserConstructionScript`)