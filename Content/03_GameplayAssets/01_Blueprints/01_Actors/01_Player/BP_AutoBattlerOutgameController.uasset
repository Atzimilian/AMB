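; Player controller for the multiplayer lobby that relays player list, ready state and match start between clients and the server.
; Server RPCs query or notify the lobby game mode, or loop over the GameState PlayerArray to push changes to every controller.
; Owning-client RPCs update the lobby widget on the HUD, including its loading screen when the match begins.
; On BeginPlay, the local controller sets Game and UI input mode.
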(event `self.ReceiveBeginPlay`
  ;[1 1 1] Only execute on local PlayerController
  (if (`self.IsLocalPlayerController`)
    ;[0.05098 0.05098 0.05098] Setup InputMode
    (`WidgetBlueprintLibrary.SetInputMode_GameAndUIEx` self null "DoNotLock" false)))

(event `ServerRPC_StartMatch`
  (for _array_element (`GameStateBase.PlayerArray` (`GameplayStatics.GetGameState`))
    (bind _asbp_auto_battler_outgame_controller (cast `/Game/03_GameplayAssets/01_Blueprints/01_Actors/01_Player/BP_AutoBattlerOutgameController` (`PlayerState.GetPlayerController` _array_element)))
    (`self.OwningClientRPC_ActivateLoadingScreen` _asbp_auto_battler_outgame_controller))
  (bind _asbp_auto_battler_lobby_mode (cast `/Game/03_GameplayAssets/06_GameSystem/02_GameModes/BP_AutoBattlerLobbyMode` (`GameplayStatics.GetGameMode`)))
  (`/Game/03_GameplayAssets/06_GameSystem/02_GameModes/BP_AutoBattlerLobbyMode.BeginMatch` _asbp_auto_battler_lobby_mode))

(event `ServerRPC_ConnectedPlayersChanged`
  (params (ConnectedPCs :type "Array of /Game/03_GameplayAssets/04_Data/01_Structs/ST_PlayerData Structure (by ref)"))
  ;[1 1 1] Update ConnectedPlayers by Server
  (for _array_element (`GameStateBase.PlayerArray` (`GameplayStatics.GetGameState`))
    (bind _asbp_auto_battler_outgame_controller (cast `/Game/03_GameplayAssets/01_Blueprints/01_Actors/01_Player/BP_AutoBattlerOutgameController` (`PlayerState.GetPlayerController` _array_element)))
    (`self.OwningClientRPC_UpdateConnectedPlayers` _asbp_auto_battler_outgame_controller ConnectedPCs)))

(event `OwningClientRPC_ActivateLoadingScreen`
  (bind _wbp_multiplayerlobby (`self.GetLobbyWidget`)
    (:`Is Valid`
      (`/Game/06_UI/01_Widgets/03_LobbyWidgets/WBP_MultiplayerLobby.StartLoadingScreen` _wbp_multiplayerlobby))))

(event `OwningClientRPC_UpdateConnectedPlayers`
  (params (ConnectedPlayers :type "Array of /Game/03_GameplayAssets/04_Data/01_Structs/ST_PlayerData Structure (by ref)"))
  ;[1 1 1] Update ConnectedPlayers by Server
  (bind _asbp_lobby_hud (cast `/Game/03_GameplayAssets/06_GameSystem/04_HUD/BP_LobbyHUD` (`self.GetHUD` self)))
  (`/Engine/EditorBlueprintResources/StandardMacros.IsValid` _asbp_lobby_hud
    (:`Is Valid`
      (bind _wbp_multiplayerlobby (`/Game/03_GameplayAssets/06_GameSystem/04_HUD/BP_LobbyHUD.WBP_MultiplayerLobby` _asbp_lobby_hud))
      (`/Engine/EditorBlueprintResources/StandardMacros.IsValid` _wbp_multiplayerlobby
        (:`Is Valid`
          (`/Game/06_UI/01_Widgets/03_LobbyWidgets/WBP_MultiplayerLobby.UpdateConnectedPlayers` _wbp_multiplayerlobby ConnectedPlayers))))))

(event `FetchConnectedPlayers`
  ;[1 1 1] Request ConnectedPlayers from Server
  (`self.ServerRPC_GatherConnectedPlayers` self))

(event `ToggleReadyState`
  (params (PlayerDataID :type Name))
  ;[1 1 1] Toggle Player Ready State
  (`self.ServerRPC_TogglePlayerReadyState` PlayerDataID))

(event `OnAllPlayersReadyState`
  (params (AreAllPlayersReady :type Boolean))
  (`self.OwningClientRPC_OnAllPlayersReadyState` AreAllPlayersReady))

(event `ServerRPC_GatherConnectedPlayers`
  (params (RequestingPlayerController :type "/Game/03_GameplayAssets/01_Blueprints/01_Actors/01_Player/BP_AutoBattlerOutgameController Object Reference"))
  ;[1 1 1] Request ConnectedPlayers from Server
  (bind _asbp_auto_battler_lobby_mode (cast `/Game/03_GameplayAssets/06_GameSystem/02_GameModes/BP_AutoBattlerLobbyMode` (`GameplayStatics.GetGameMode`)))
  (`self.OwningClientRPC_UpdateConnectedPlayers` RequestingPlayerController (`/Game/03_GameplayAssets/06_GameSystem/02_GameModes/BP_AutoBattlerLobbyMode.ConnectedPlayers` _asbp_auto_battler_lobby_mode)))

(event `ServerRPC_TogglePlayerReadyState`
  (params (PlayerDataID :type Name))
  ;[1 1 1] Toggle Player Ready State
  (bind _asbp_auto_battler_lobby_mode (cast `/Game/03_GameplayAssets/06_GameSystem/02_GameModes/BP_AutoBattlerLobbyMode` (`GameplayStatics.GetGameMode`)))
  (`/Game/03_GameplayAssets/06_GameSystem/02_GameModes/BP_AutoBattlerLobbyMode.OnPlayerReadyStateChange` _asbp_auto_battler_lobby_mode PlayerDataID))

(event `OwningClientRPC_OnAllPlayersReadyState`
  (params (AreAllPlayersReady :type Boolean))
  (bind _wbp_multiplayerlobby (`self.GetLobbyWidget`)
    (:`Is Valid`
      (`/Game/06_UI/01_Widgets/03_LobbyWidgets/WBP_MultiplayerLobby.UpdateAllPlayerReadyState` _wbp_multiplayerlobby AreAllPlayersReady))))

(event `ServerRPC_UpdatePlayerReadyState`
  (params (UpdatedPlayerData :type "/Game/03_GameplayAssets/04_Data/01_Structs/ST_PlayerData Structure"))
  ;[1 1 1] Player changed Ready State
  (for _array_element (`GameStateBase.PlayerArray` (`GameplayStatics.GetGameState`))
    (bind _asbp_auto_battler_outgame_controller (cast `/Game/03_GameplayAssets/01_Blueprints/01_Actors/01_Player/BP_AutoBattlerOutgameController` (`PlayerState.GetPlayerController` _array_element)))
    (`self.OwningClientRPC_OnPlayerReadyStateChange` _asbp_auto_battler_outgame_controller UpdatedPlayerData)))

(event `OwningClientRPC_OnPlayerReadyStateChange`
  (params (UpdatedPlayerData :type "/Game/03_GameplayAssets/04_Data/01_Structs/ST_PlayerData Structure"))
  ;[1 1 1] Player changed Ready State
  (bind _wbp_multiplayerlobby (`self.GetLobbyWidget`)
    (:`Is Valid`
      (`/Game/06_UI/01_Widgets/03_LobbyWidgets/WBP_MultiplayerLobby.UpdatePlayerReadyState` _wbp_multiplayerlobby UpdatedPlayerData))))

(fn `UserConstructionScript`
  (`parent.UserConstructionScript`))