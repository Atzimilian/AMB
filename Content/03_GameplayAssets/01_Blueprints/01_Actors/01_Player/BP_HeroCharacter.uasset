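; Player hero character for the auto battler, providing an RTS-style camera through Enhanced Input.
; The construction script detaches the SpringArm, which input then moves for panning, with an optional speed boost.
; Scrolling changes the clamped arm length, and a zoom-based factor scales pan and scroll speeds.
; Screen-edge panning with a dead zone is present but disconnected, so it never runs.
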(event `self.ReceiveBeginPlay`
  ;[1 1 1] Setup Enhanced Input Control
  (bind _asbp_auto_battler_ingame_controller (cast `/Game/03_GameplayAssets/01_Blueprints/01_Actors/01_Player/BP_AutoBattlerIngameController` (`self.GetController`)))
  (bind _returnvalue (pcsubsystem `EnhancedInputLocalPlayerSubsystem` _asbp_auto_battler_ingame_controller))
  (`/Engine/EditorBlueprintResources/StandardMacros.IsValid` _returnvalue
    (:`Is Valid`
      (`EnhancedInputSubsystemInterface.AddMappingContext` _returnvalue "/Game/08_Input/IMC_RTSDefault.IMC_RTSDefault" 0 (struct)))))

(event `EnhancedInput|/Game/08_Input/IA_MovePaning`
  (params (ActionValue :type "Vector2D Structure") (ElapsedSeconds :type "Float (double-precision)") (TriggeredSeconds :type "Float (double-precision)") (InputAction :type "InputAction Object Reference" :default "/Game/08_Input/IA_MovePaning.IA_MovePaning"))
  ;[1 1 1] Camera Movement
  (:`Triggered`
    (`self.PanMoveCamera` ActionValue (* (`self.panSpeed`) (`self.GetZoomSpeedFactor`)) true)))

(event `InputAxisKey|MouseX`
  (params (AxisValue :type "Float (single-precision)"))
  ;[1 1 1] Camera Movement
)

(event `EnhancedInput|/Game/08_Input/IA_ScrollHeight`
  (params (ActionValue :type "Float (double-precision)") (ElapsedSeconds :type "Float (double-precision)") (TriggeredSeconds :type "Float (double-precision)") (InputAction :type "InputAction Object Reference" :default "/Game/08_Input/IA_ScrollHeight.IA_ScrollHeight"))
  ;[1 1 1] Camera Movement
  (:`Triggered`
    (`self.ZoomCamera` ActionValue)))

(event `EnhancedInput|/Game/08_Input/IA_BoostPanning`
  (params (ActionValue :type Boolean) (ElapsedSeconds :type "Float (double-precision)") (TriggeredSeconds :type "Float (double-precision)") (InputAction :type "InputAction Object Reference" :default "/Game/08_Input/IA_BoostPanning.IA_BoostPanning"))
  ;[1 1 1] Camera Movement
  (:`Started`
    (set `self.isBoostPanning` true))
  (:`Completed`
    (set `self.isBoostPanning` false)))

(fn `PanMoveCamera`
  (params (`In XY-Axis` :type "Vector2D Structure") (MoveSpeed :type "Float (double-precision)") (CanBoostSpeed :type Boolean))
  (bind _springarm (`self.SpringArm`))
  (`SceneComponent.K2_SetRelativeLocation` _springarm (+ (`SceneComponent.RelativeLocation` _springarm) (* (`KismetMathLibrary.Normal2D` `In XY-Axis`) (* (`KismetMathLibrary.SelectFloat` (`self.panBoostFactor`) 1.0 (and (`self.isBoostPanning`) CanBoostSpeed)) MoveSpeed (`GameplayStatics.GetWorldDeltaSeconds`)))) false false))

(fn `UserConstructionScript`
  (`SceneComponent.K2_DetachFromComponent` (`self.SpringArm`) "KeepWorld" "KeepWorld" "KeepWorld" true))

(fn `ZoomCamera`
  (params (`In Scroll Axis` :type "Float (double-precision)"))
  (bind _springarm (`self.SpringArm`))
  (set `SpringArmComponent.TargetArmLength` (`KismetMathLibrary.FMin` (`KismetMathLibrary.FMax` (+ (`SpringArmComponent.TargetArmLength` _springarm) (* (* (* `In Scroll Axis` -1.0) (* (`self.scrollSpeed`) (`self.GetZoomSpeedFactor`))) (`GameplayStatics.GetWorldDeltaSeconds`))) (`self.minScrollHeight`)) (`self.maxScrollHeight`)) _springarm))