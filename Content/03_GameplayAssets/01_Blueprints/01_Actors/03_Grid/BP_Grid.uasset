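; BP_Grid is a grid actor that spawns a rectangular field of square child actors.
; BuildGrid loops over GridSize and adds a child actor component per cell, spacing cells by the SquareClass default SquareSize plus GridGap and centring them on the actor.
; It branches on IsLocalPlayer, with both branches using identical placement.
; The construction script is empty, with its BuildGrid call left disconnected.
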(fn `BuildGrid`
  (params (IsLocalPlayer :type Boolean))
  (locals (HalfSizeX :type "Float (double-precision)") (HalfSizeY :type "Float (double-precision)"))
  (bind (_gridsize_x _gridsize_y) (`KismetMathLibrary.BreakVector2D` (`self.GridSize`)))
  (bind (_gridsize_x_2 _gridsize_y_2) (`KismetMathLibrary.BreakVector2D` (`self.GridSize`)))
  (bind _returnvalue (+ (defaults `Object` (`self.SquareClass`)) (`self.GridGap`)))
  (bind _returnvalue_2 (+ (defaults `Object` (`self.SquareClass`)) (`self.GridGap`)))
  (bind _returnvalue_3 (* (+ (`self.GridGap`) (defaults `Object` (`self.SquareClass`))) 0.5))
  (set `local.HalfSizeX` (- (* _gridsize_x _returnvalue_2 0.5) _returnvalue_3 0.0))
  (set `local.HalfSizeY` (- (* _gridsize_y _returnvalue_2 0.5) _returnvalue_3 0.0))
  (for _index (range (+ (`KismetMathLibrary.FTrunc` (- _gridsize_x_2 1.0)) 1))
    (for _index_2 (range (+ (`KismetMathLibrary.FTrunc` (- _gridsize_y_2 1.0)) 1))
      (if (`local.IsLocalPlayer`)
        (bind _returnvalue_4 (- (* _index _returnvalue) (`local.HalfSizeX`)))
        (bind _returnvalue_5 (- (* _index_2 _returnvalue) (`local.HalfSizeY`)))
        (`AddComponent|NODE_AddChildActorComponent-0` :`RelativeTransform` (`KismetMathLibrary.MakeTransform` (`KismetMathLibrary.MakeVector` _returnvalue_4 _returnvalue_5)))
        (else
          (`AddComponent|NODE_AddChildActorComponent-1` :`RelativeTransform` (`KismetMathLibrary.MakeTransform` (`KismetMathLibrary.MakeVector` _returnvalue_4 _returnvalue_5))))))))

(fn `UserConstructionScript`)