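; BP_Square is a grid square actor with a static mesh and a box component, sized by its SquareSize variable.
; The construction script scales the mesh and box extent in X and Y by SquareSize relative to 100 units, leaving height unchanged.
; It then lifts both components by half their height so they rest on the actor's origin, assuming a centred 100-unit mesh.
; The event graph holds no gameplay logic.
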(fn `UserConstructionScript`
  (bind _staticmesh (`self.StaticMesh`))
  (bind _staticmesh_2 (`self.StaticMesh`))
  (bind _box (`self.Box`))
  (bind _returnvalue (/ (`self.squareSize`) 100.0))
  (bind _returnvalue_2 (/ (`self.squareSize`) 100.0))
  (bind (_boxextent_x _boxextent_y _boxextent_z) (`KismetMathLibrary.BreakVector` (`BoxComponent.BoxExtent` _box)))
  (bind (_relativescale3d_x _relativescale3d_y _relativescale3d_z) (`KismetMathLibrary.BreakVector` (`SceneComponent.RelativeScale3D` _staticmesh_2)))
  (bind (_relativescale3d_x_2 _relativescale3d_y_2 _relativescale3d_z_2) (`KismetMathLibrary.BreakVector` (`SceneComponent.RelativeScale3D` _staticmesh)))
  (`SceneComponent.SetRelativeScale3D` _staticmesh (`KismetMathLibrary.MakeVector` _returnvalue _returnvalue _relativescale3d_z_2))
  (`SceneComponent.K2_SetRelativeLocation` _staticmesh_2 (`KismetMathLibrary.MakeVector` 0.0 0.0 (/ (* _relativescale3d_z 100.0) 2.0)) false false)
  (`BoxComponent.SetBoxExtent` _box (`KismetMathLibrary.MakeVector` (* _returnvalue_2 _boxextent_x) (* _returnvalue_2 _boxextent_y) _boxextent_z) true)
  (`SceneComponent.K2_SetRelativeLocation` _box (`KismetMathLibrary.MakeVector` 0.0 0.0 _boxextent_z) false false))