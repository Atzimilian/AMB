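; Player build island actor for an auto battler, tied to an assigned player index that it exposes through a getter.
; On BeginPlay it spawns an owned BP_Grid at the transform of its BPBattleGrid and stores the reference.
; It then builds that grid outside preview mode, flagged as local when the first player controller's own slot index matches the island's assigned index.
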(event `self.ReceiveBeginPlay`
  (`self.ConstructGrid`))

(fn `ConstructGrid`
  (bind _returnvalue (`|SpawnActorFromClass` "/Game/03_GameplayAssets/01_Blueprints/01_Actors/03_Grid/BP_Grid.BP_Grid_C" (`SceneComponent.K2_GetComponentToWorld` (`self.BP_BattleGrid`)) "AlwaysSpawn" "OverrideRootScale" self null))
  (set `self.BP_Grid` _returnvalue)
  (bind _asbp_auto_battler_ingame_controller (cast `/Game/03_GameplayAssets/01_Blueprints/01_Actors/01_Player/BP_AutoBattlerIngameController` (`GameplayStatics.GetPlayerController` 0)))
  (if true
    (`/Game/03_GameplayAssets/01_Blueprints/01_Actors/03_Grid/BP_Grid.BuildGrid` (`self.BP_Grid`) (== (`.PlayerSlotIndex_19_821D2B7B47D671A0AD0677A89D4D41D4` (break `/Game/03_GameplayAssets/04_Data/01_Structs/ST_PlayerData` (`/Game/03_GameplayAssets/01_Blueprints/01_Actors/01_Player/BP_AutoBattlerIngameController.OwnPlayerData` _asbp_auto_battler_ingame_controller))) (`self.AssignedPlayerIndex`)) false)))

(fn `GetAssignedPlayerIndex`
  (returns (AssignedPlayerIndex :type Integer))
  (return (`self.AssignedPlayerIndex`)))

(fn `UserConstructionScript`)