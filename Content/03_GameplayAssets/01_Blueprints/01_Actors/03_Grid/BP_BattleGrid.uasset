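; BP_BattleGrid is a battle grid actor that, as shown, only sizes a preview box and spawns no squares.
; Its construction script sets the PreviewSize box extent from CalcHalfXYSize and raises it to sit above the origin.
; CalcHalfXYSize contains half-span formulas from GridSize, GridGap and BP_Square's default SquareSize, but they appear unconnected to its outputs.
; The event graph holds only empty placeholder events.
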(fn `UserConstructionScript`
  (bind (_halfxsize _halfysize) (`self.CalcHalfXYSize`))
  (`BoxComponent.SetBoxExtent` (`self.PreviewSize`) (`KismetMathLibrary.MakeVector` _halfxsize _halfysize 100.0) true)
  (`SceneComponent.K2_SetRelativeLocation` (`self.PreviewSize`) (0.0 0.0 100.0) false false))