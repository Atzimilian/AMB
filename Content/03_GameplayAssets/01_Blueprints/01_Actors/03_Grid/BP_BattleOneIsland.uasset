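; Battle island actor that runs and scores one fight between two player armies on two grids.
; It spawns units from army data, makes each side the other's AI target list and toggles their AI combat.
; Death events track casualties until one army is wiped out, then combat stops and evaluation picks a winner, with remaining-percentage tie-break.
; Kill points and rank-weighted lost health are broadcast once, and the game state is notified.
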(event `ReturnBattleOutcome`
  (params (IslandOutcome :type "/Game/03_GameplayAssets/04_Data/01_Structs/ST_BattleOutcome Structure") (PlayerAResult :type "/Game/03_GameplayAssets/04_Data/01_Structs/ST_BattleResult Structure") (PlayerBResult :type "/Game/03_GameplayAssets/04_Data/01_Structs/ST_BattleResult Structure"))
  (`self.BattleOutcome` IslandOutcome PlayerAResult PlayerBResult))

(fn `AssignPlayerArmies`
  (params (PlayerArmyA :type "Array of /Game/03_GameplayAssets/04_Data/01_Structs/ST_PlayerUnit Structure") (PlayerArmyB :type "Array of /Game/03_GameplayAssets/04_Data/01_Structs/ST_PlayerUnit Structure"))
  (`KismetArrayLibrary.Array_Clear` (`self.KilledUnitsPlayerA`))
  (`KismetArrayLibrary.Array_Clear` (`self.KilledUnitsPlayerB`))
  (`KismetArrayLibrary.Array_Clear` (`self.PlayerArmyA`))
  (`KismetArrayLibrary.Array_Clear` (`self.PlayerArmyB`))
  (set `self.PlayerArmyA` PlayerArmyA)
  (set `self.PlayerArmyB` PlayerArmyB))

(fn `BattleFinished`
  (`self.StopBattleUnitsCombat`)
  (`self.EvaluateMatch`)
  (`/Game/03_GameplayAssets/06_GameSystem/03_GameStates/BP_AMB_IngameState.BattleIslandFinished` (`/Game/03_GameplayAssets/01_Blueprints/90_MacroLibs/BPFL_GetGameSystem.GetAMBIngameState`)))

(fn `CalculateKillPoints`
  (params (KilledUnits :type "Array of DataTableRowHandle Structure"))
  (returns (KP :type Integer) (TopRank :type Integer))
  (locals (KillPoints :type Integer) (MaxRank :type Integer :default 0))
  ;[1 1 1] Base * Unit Upgrade Level) Killpoints
  (for _array_element KilledUnits
    (bind _returnvalue (`|GetDataTableRow` "/Game/03_GameplayAssets/04_Data/03_DataTables/DT_UnitStats.DT_UnitStats" (`.RowName` (break `DataTableRowHandle` _array_element)))
      (:`then`
        (bind ((`Rank_27_9197347C41DB31474F6CA1AC08C0B1A9` _rank)) (break `/Game/03_GameplayAssets/04_Data/01_Structs/ST_Unit_Stats` _returnvalue))
        (set `local.KillPoints` (+ (+ _rank 1) (`local.KillPoints`)))
        (if (> _rank (`local.MaxRank`))
          (bind _output_get (set `local.MaxRank` _rank))))))
  (return (`local.KillPoints`) _output_get))

(fn `CleanUpBattle`
  (`|ExecutionSequence`
    (:`then_0`
      (for _array_element (`self.PlayerArmyAUnits`)
        (`/Engine/EditorBlueprintResources/StandardMacros.IsValid` _array_element
          (:`Is Valid`
            (`self.K2_DestroyActor` _array_element)
            (set `self.PlayerASlotIndex` -1)))))
    (:`then_1`
      (for _array_element_2 (`self.PlayerArmyBUnits`)
        (`/Engine/EditorBlueprintResources/StandardMacros.IsValid` _array_element_2
          (:`Is Valid`
            (`self.K2_DestroyActor` _array_element_2)
            (set `self.PlayerBSlotIndex` -1)))))
    (:`then_2`
      (`KismetArrayLibrary.Array_Clear` (`self.PlayerArmyAUnits`))
      (`KismetArrayLibrary.Array_Clear` (`self.PlayerArmyBUnits`))
      (`KismetArrayLibrary.Array_Clear` (`self.KilledUnitsPlayerA`))
      (`KismetArrayLibrary.Array_Clear` (`self.KilledUnitsPlayerB`))
      (`KismetArrayLibrary.Array_Clear` (`self.PlayerArmyA`))
      (`KismetArrayLibrary.Array_Clear` (`self.PlayerArmyB`)))))

(fn `DebugSpawnUnits`
  (bind _asbp_amb_ingame_state (`/Game/03_GameplayAssets/01_Blueprints/90_MacroLibs/BPFL_GetGameSystem.GetAMBIngameState`))
  (bind _ingameplayerdata (`/Game/03_GameplayAssets/06_GameSystem/03_GameStates/BP_AMB_IngameState.IngamePlayerData` _asbp_amb_ingame_state))
  (`|ExecutionSequence`
    (:`then_0`
      (bind _output_get (set `self.PlayerASlotIndex` (`.PlayerSlotIndex_19_821D2B7B47D671A0AD0677A89D4D41D4` (break `/Game/03_GameplayAssets/04_Data/01_Structs/ST_PlayerData` (`|GetArrayItem` _ingameplayerdata)))))
      (bind _outplayerowningunits (`/Game/03_GameplayAssets/06_GameSystem/03_GameStates/BP_AMB_IngameState.GetPlayerUnitsOfPlayerSlotIndex` _asbp_amb_ingame_state _output_get))
      (set `self.PlayerArmyA` _outplayerowningunits))
    (:`then_1`
      (if (> (`KismetArrayLibrary.Array_Length` _ingameplayerdata) 1)
        (bind _output_get_2 (set `self.PlayerBSlotIndex` (`.PlayerSlotIndex_19_821D2B7B47D671A0AD0677A89D4D41D4` (break `/Game/03_GameplayAssets/04_Data/01_Structs/ST_PlayerData` (`|GetArrayItem` _ingameplayerdata 1)))))
        (bind _outplayerowningunits_2 (`/Game/03_GameplayAssets/06_GameSystem/03_GameStates/BP_AMB_IngameState.GetPlayerUnitsOfPlayerSlotIndex` _asbp_amb_ingame_state _output_get_2))
        (set `self.PlayerArmyB` _outplayerowningunits_2)
        (else
          (set `self.PlayerArmyB` _outplayerowningunits))))
    (:`then_2`
      (`self.PrepareBattle`))))

(fn `EvaluateMatch`
  (locals (`Player B Remaining Units` :type Integer) (`Player A Remaining Units` :type Integer) (`Player A Starting Units` :type Integer) (`Player B Starting Units` :type Integer) (`Player A Kill Points` :type Integer) (`Player B Kill Points` :type Integer) (`Player A MaxRank` :type Integer) (`Player B MaxRank` :type Integer) (`Player A LostHealth` :type Integer) (`Player B LostHealth` :type Integer))
  (`|ExecutionSequence`
    (:`then_0`
      ;[0.2726 0.2726 0.2726] Determine Winner
      ;;[1 1 1] Initialize kill points to 0
      (`self.ResetKillPoints`)
      (`self.SetStartingUnitsPlayerA`)
      (`self.SetRemainingUnitsPlayerA`)
      (`self.SetStartingUnitsPlayerB`)
      (`self.SetRemainingUnitsPlayerB`)
      (if (== (`local.Player B Remaining Units`) 0)
        ;;[1 1 1] Simple Win Case
        (set `self.PlayerAWin` true)
        (elif (== (`local.Player A Remaining Units`) 0)
          (set `self.PlayerAWin` false)
          (else
            ;;[1 1 1] Tie Break Win Case
            (if (>= (/ (`local.Player A Remaining Units`) (`local.Player A Starting Units`)) (/ (`local.Player B Remaining Units`) (`local.Player B Starting Units`)))
              (set `self.PlayerAWin` true)
              (else
                (set `self.PlayerAWin` false)))))))
    (:`then_1`
      ;[1 1 1] Calculate Kill Points and max rank for both teams
      (bind (_kp _toprank) (`self.CalculateKillPoints` (`self.KilledUnitsPlayerB`)))
      (set `local.Player A Kill Points` _kp)
      (set `local.Player A MaxRank` _toprank))
    (:`then_2`
      (bind (_kp_2 _toprank_2) (`self.CalculateKillPoints` (`self.KilledUnitsPlayerA`)))
      (set `local.Player B Kill Points` _kp_2)
      (set `local.Player B MaxRank` _toprank_2))
    (:`then_3`
      ;[1 1 1] Calculate Lost Health = (looser lost units)*highest rank + (winner surviving units)highest rank
      (if (`self.PlayerAWin`)
        (set `local.Player A LostHealth` 0)
        (set `local.Player B LostHealth` (+ (* (- (`local.Player B Starting Units`) (`local.Player B Remaining Units`)) (`local.Player B MaxRank`)) (* (`local.Player A Remaining Units`) (`local.Player A MaxRank`))))
        (else
          (set `local.Player B LostHealth` 0)
          (set `local.Player A LostHealth` (+ (* (- (`local.Player A Starting Units`) (`local.Player A Remaining Units`)) (`local.Player A MaxRank`)) (* (`local.Player B Remaining Units`) (`local.Player B MaxRank`)))))))
    (:`then_4`
      (if (not (`self.Evaluated`))
        (`self.ReturnBattleOutcome` (make `/Game/03_GameplayAssets/04_Data/01_Structs/ST_BattleOutcome` (`self.PlayerAWin`) (`local.Player A Starting Units`) (`local.Player B Starting Units`) (`local.Player A Remaining Units`) (`local.Player B Remaining Units`) (`local.Player A Kill Points`) (`local.Player B Kill Points`) 0 (`self.PlayerASlotIndex`) (`self.PlayerBSlotIndex`)) (make `/Game/03_GameplayAssets/04_Data/01_Structs/ST_BattleResult` (`self.PlayerAWin`) (`local.Player A Kill Points`) (`local.Player A Remaining Units`) (`local.Player A LostHealth`) (`KismetArrayLibrary.Array_Length` (`self.KilledUnitsPlayerB`)) (`self.PlayerASlotIndex`)) (make `/Game/03_GameplayAssets/04_Data/01_Structs/ST_BattleResult` (not (`self.PlayerAWin`)) (`local.Player B Kill Points`) (`local.Player B Remaining Units`) (`local.Player B LostHealth`) (`KismetArrayLibrary.Array_Length` (`self.KilledUnitsPlayerA`)) (`self.PlayerBSlotIndex`)))))
    (:`then_5`
      ;[1 1 1] Confirm Island has been Evaluated
      (set `self.Evaluated` true))))

(fn `GetWinningPlayerRemainingUnits`
  (returns (WiningPlayerRemainingUnits :type "Array of /Game/03_GameplayAssets/04_Data/01_Structs/ST_PlayerUnit Structure") (WinningPlayerSlotIndex :type Integer) (DidPlayerAWin :type Boolean))
  (locals (RemainingPlayerUnits :type "Array of /Game/03_GameplayAssets/04_Data/01_Structs/ST_PlayerUnit Structure"))
  (bind _returnvalue (`KismetMathLibrary.SelectInt` (`self.PlayerASlotIndex`) (`self.PlayerBSlotIndex`) (`self.PlayerAWin`)))
  (`KismetArrayLibrary.Array_Clear` (`local.RemainingPlayerUnits`))
  (for _array_element (select `bool` (`self.PlayerAWin`) :`false` (`self.PlayerArmyBUnits`) :`true` (`self.PlayerArmyAUnits`))
    (bind (_buildgridposition_xindex _buildgridposition_yindex) (break `/Game/03_GameplayAssets/04_Data/01_Structs/ST_GridCoords` (`/Game/03_GameplayAssets/01_Blueprints/01_Actors/02_Unit/BP_Unit.BuildGridPosition` _array_element)))
    (bind (_unitdatarow_datatable _unitdatarow_rowname) (break `DataTableRowHandle` (`/Game/03_GameplayAssets/01_Blueprints/01_Actors/02_Unit/BP_Unit.UnitDataRow` _array_element)))
    (`KismetArrayLibrary.Array_Add` (`local.RemainingPlayerUnits`) (make `/Game/03_GameplayAssets/04_Data/01_Structs/ST_PlayerUnit` _returnvalue _buildgridposition_xindex _buildgridposition_yindex _unitdatarow_rowname)))
  (return (`local.RemainingPlayerUnits`) _returnvalue (`self.PlayerAWin`)))

(fn `KilledUnitCheck`
  (bind _returnvalue (== (`KismetArrayLibrary.Array_Length` (`self.PlayerArmyB`)) (`KismetArrayLibrary.Array_Length` (`self.KilledUnitsPlayerB`))))
  (if (or _returnvalue (== (`KismetArrayLibrary.Array_Length` (`self.PlayerArmyA`)) (`KismetArrayLibrary.Array_Length` (`self.KilledUnitsPlayerA`))))
    (set `self.PlayerAWin` _returnvalue)
    (`self.BattleFinished`)))

(fn `On Unit ADeath`
  (params (RefToDeadUnit :type "/Game/03_GameplayAssets/01_Blueprints/01_Actors/02_Unit/BP_Unit Object Reference") (OwningPlayerSlotIndex :type Integer) (KillerPlayerSlotIndex :type Integer))
  (`KismetArrayLibrary.Array_Add` (`self.KilledUnitsPlayerA`) (`/Game/03_GameplayAssets/01_Blueprints/01_Actors/02_Unit/BP_Unit.UnitDataRow` RefToDeadUnit))
  (`KismetArrayLibrary.Array_RemoveItem` (`self.PlayerArmyAUnits`) RefToDeadUnit)
  (`self.KilledUnitCheck`))

(fn `OnUnitBDeath`
  (params (RefToDeadUnit :type "/Game/03_GameplayAssets/01_Blueprints/01_Actors/02_Unit/BP_Unit Object Reference") (OwningPlayerSlotIndex :type Integer) (KillerPlayerSlotIndex :type Integer))
  (`KismetArrayLibrary.Array_Add` (`self.KilledUnitsPlayerB`) (`/Game/03_GameplayAssets/01_Blueprints/01_Actors/02_Unit/BP_Unit.UnitDataRow` RefToDeadUnit))
  (`KismetArrayLibrary.Array_RemoveItem` (`self.PlayerArmyBUnits`) RefToDeadUnit)
  (`self.KilledUnitCheck`))

(fn `PrepareBattle`
  (locals (CurrentOwningPlayerController :type "/Game/03_GameplayAssets/01_Blueprints/01_Actors/01_Player/BP_AutoBattlerPlayerController Object Reference"))
  (set `self.Evaluated` false)
  (`|ExecutionSequence`
    (:`then_0`
      (if (>= (`self.PlayerASlotIndex`) 0)
        (`self.SpawnPlayerBattleUnit` null (`self.PlayerArmyA`) (`self.PlayerASlotIndex`) (`self.PlayerArmyAUnits`) (`self.BattleGridA`) (`|CreateDelegate` :!event `On Unit ADeath`))))
    (:`then_1`
      (if (>= (`self.PlayerBSlotIndex`) 0)
        (`self.SpawnPlayerBattleUnit` null (`self.PlayerArmyB`) (`self.PlayerBSlotIndex`) (`self.PlayerArmyBUnits`) (`self.BattleGridB`) (`|CreateDelegate` :!event `OnUnitBDeath`))))
    (:`then_2`
      (`self.SetupTargetLists`))))

(fn `SetupTargetLists`
  (`|ExecutionSequence`
    (:`then_0`
      (for _array_element (`self.PlayerArmyAUnits`)
        (bind _asbp_unit_ai_controller (cast `/Game/03_GameplayAssets/05_AI/BP_Unit_AI_Controller` (`AIBlueprintHelperLibrary.GetAIController` _array_element)))
        (set `/Game/03_GameplayAssets/05_AI/BP_Unit_AI_Controller.TargetList` (`self.PlayerArmyBUnits`) _asbp_unit_ai_controller)))
    (:`then_1`
      (for _array_element_2 (`self.PlayerArmyBUnits`)
        (bind _asbp_unit_ai_controller_2 (cast `/Game/03_GameplayAssets/05_AI/BP_Unit_AI_Controller` (`AIBlueprintHelperLibrary.GetAIController` _array_element_2)))
        (set `/Game/03_GameplayAssets/05_AI/BP_Unit_AI_Controller.TargetList` (`self.PlayerArmyAUnits`) _asbp_unit_ai_controller_2)))))

(fn `SpawnPlayerBattleUnit`
  (params (OwningPlayerController :type "/Game/03_GameplayAssets/01_Blueprints/01_Actors/01_Player/BP_AutoBattlerIngameController Object Reference") (PlayerBattleUnits :type "Array of /Game/03_GameplayAssets/04_Data/01_Structs/ST_PlayerUnit Structure") (PlayerSlotIndex :type Integer) (PlayerUnitsActor :type "Array of /Game/03_GameplayAssets/01_Blueprints/01_Actors/02_Unit/BP_Unit Object Reference") (`Battle Grid` :type "SceneComponent Object Reference") (OnUnitDeathEvent :type "Delegate (by ref)"))
  (bind _battle_grid (`local.Battle Grid`))
  (for _array_element PlayerBattleUnits
    (bind _returnvalue (`|SpawnActorFromClass` "/Game/03_GameplayAssets/01_Blueprints/01_Actors/02_Unit/BP_Unit.BP_Unit_C" (`KismetMathLibrary.MakeTransform` (`KismetMathLibrary.TransformLocation` (`SceneComponent.K2_GetComponentToWorld` _battle_grid) (`self.GetUnitSpawnPos` (`.GridX_9_6E6FE8F7450C0AF2A19728A673713AF8` (break `/Game/03_GameplayAssets/04_Data/01_Structs/ST_PlayerUnit` _array_element)) (`.GridY_8_4408DBD041F6E1D80DBD51BFF2B0C40F` (break `/Game/03_GameplayAssets/04_Data/01_Structs/ST_PlayerUnit` _array_element)) (`SceneComponent.K2_GetComponentLocation` _battle_grid))) (`SceneComponent.K2_GetComponentRotation` _battle_grid)) "AlwaysSpawn" "MultiplyWithRoot" null null))
    (`KismetArrayLibrary.Array_Add` (`local.PlayerUnitsActor`) _returnvalue)
    (set `/Game/03_GameplayAssets/01_Blueprints/01_Actors/02_Unit/BP_Unit.BuildGridPosition` (make `/Game/03_GameplayAssets/04_Data/01_Structs/ST_GridCoords` (`.GridX_9_6E6FE8F7450C0AF2A19728A673713AF8` (break `/Game/03_GameplayAssets/04_Data/01_Structs/ST_PlayerUnit` _array_element)) (`.GridY_8_4408DBD041F6E1D80DBD51BFF2B0C40F` (break `/Game/03_GameplayAssets/04_Data/01_Structs/ST_PlayerUnit` _array_element))) _returnvalue)
    (set `/Game/03_GameplayAssets/01_Blueprints/01_Actors/02_Unit/BP_Unit.PlayerSlotIndex` PlayerSlotIndex _returnvalue)
    (set `/Game/03_GameplayAssets/01_Blueprints/01_Actors/02_Unit/BP_Unit.UnitDataRow` (make `DataTableRowHandle` "/Game/03_GameplayAssets/04_Data/03_DataTables/DT_Units.DT_Units" (`.UnitType_RowName_7_79D49A6D41D3B1C19FE681A3634D2CA7` (break `/Game/03_GameplayAssets/04_Data/01_Structs/ST_PlayerUnit` _array_element))) _returnvalue)
    (`/Game/03_GameplayAssets/01_Blueprints/01_Actors/02_Unit/BP_Unit.SetStatsByDTRowName` _returnvalue (`.UnitStats_RowName_15_0888446B4F8990BF29F2E3AB4B58AA35` (break `/Game/03_GameplayAssets/04_Data/01_Structs/ST_PlayerUnit` _array_element)))
    (`/Game/03_GameplayAssets/01_Blueprints/01_Actors/02_Unit/BP_Unit.SetBattleUnit` _returnvalue true)
    (add `/Game/03_GameplayAssets/01_Blueprints/01_Actors/02_Unit/BP_Unit.OnUnitDeath` _returnvalue OnUnitDeathEvent)))

(fn `StartBattleUnitsCombat`
  (`|ExecutionSequence`
    (:`then_0`
      (for _array_element (`self.PlayerArmyAUnits`)
        (bind _asbp_unit_ai_controller (cast `/Game/03_GameplayAssets/05_AI/BP_Unit_AI_Controller` (`AIBlueprintHelperLibrary.GetAIController` _array_element)))
        (`/Game/03_GameplayAssets/05_AI/BP_Unit_AI_Controller.StartAI` _asbp_unit_ai_controller)))
    (:`then_1`
      (for _array_element_2 (`self.PlayerArmyBUnits`)
        (bind _asbp_unit_ai_controller_2 (cast `/Game/03_GameplayAssets/05_AI/BP_Unit_AI_Controller` (`AIBlueprintHelperLibrary.GetAIController` _array_element_2)))
        (`/Game/03_GameplayAssets/05_AI/BP_Unit_AI_Controller.StartAI` _asbp_unit_ai_controller_2)))))

(fn `StopBattleUnitsCombat`
  (`|ExecutionSequence`
    (:`then_0`
      (for _array_element (`self.PlayerArmyAUnits`)
        (bind _asbp_unit_ai_controller (cast `/Game/03_GameplayAssets/05_AI/BP_Unit_AI_Controller` (`AIBlueprintHelperLibrary.GetAIController` _array_element)))
        (`/Game/03_GameplayAssets/05_AI/BP_Unit_AI_Controller.StopAI` _asbp_unit_ai_controller)))
    (:`then_1`
      (for _array_element_2 (`self.PlayerArmyBUnits`)
        (bind _asbp_unit_ai_controller_2 (cast `/Game/03_GameplayAssets/05_AI/BP_Unit_AI_Controller` (`AIBlueprintHelperLibrary.GetAIController` _array_element_2)))
        (`/Game/03_GameplayAssets/05_AI/BP_Unit_AI_Controller.StopAI` _asbp_unit_ai_controller_2)))))

(fn `UserConstructionScript`)