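; BP_AudioManager is an audio manager Blueprint that relays requests to play sound effects at a world location across the network.
; A server event calls a multicast event, which in turn calls a client event that plays the sound, with debug prints at each hop.
; The client event switches on the sound type, setting a named integer parameter only for the attack cue; death and shop-sell cases add nothing.
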(event `RPC_Server_PlaySoundAtLocation`
  (params (Sound :type "/Game/03_GameplayAssets/04_Data/02_Enums/E_Audio_Cues Enum" :default "NewEnumerator0") (Location :type "Vector Structure") (ParamInt :type Integer) (ParamName :type Name))
  (`self.RPC_Multicast_PlaySoundAtLocation` Sound Location ParamInt ParamName)
  (`KismetSystemLibrary.PrintString` "murticast called from server"))

(event `RPC_Multicast_PlaySoundAtLocation`
  (params (Sound :type "/Game/03_GameplayAssets/04_Data/02_Enums/E_Audio_Cues Enum" :default "NewEnumerator0") (Location :type "Vector Structure") (ParamInt :type Integer) (ParamName :type Name))
  (`self.RPC_Client_PlaySoundAtLocation` Sound Location ParamInt ParamName)
  (`KismetSystemLibrary.PrintString` "client called from multicast"))

(event `RPC_Client_PlaySoundAtLocation`
  (params (Sound :type "/Game/03_GameplayAssets/04_Data/02_Enums/E_Audio_Cues Enum" :default "NewEnumerator0") (Location :type "Vector Structure") (ParamInt :type Integer) (ParamName :type Name))
  (switch `/Game/03_GameplayAssets/04_Data/02_Enums/E_Audio_Cues` Sound
    (:`NewEnumerator0`
      (`AudioParameterControllerInterface.SetIntParameter` (`self.AttackSFXCue`) ParamName ParamInt))
    (:`NewEnumerator1`
      _)
    (:`NewEnumerator2`
      _))
  (`GameplayStatics.PlaySoundAtLocation` null Location (struct) 1.0 1.0 0.0 null null null null)
  (`KismetSystemLibrary.PrintString` "sound played at location"))

(fn `UserConstructionScript`)