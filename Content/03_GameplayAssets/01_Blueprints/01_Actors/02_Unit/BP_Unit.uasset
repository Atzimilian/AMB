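; Auto-battler unit pawn that fights, shows health, rank and player colour, and can be dragged and placed on board squares.
; DT_UnitStats and DT_Units rows drive stats, mesh, animations and upgrade lookup, with RepNotifies refreshing visuals.
; Server-side attacks roll crits on an attack-speed cooldown and queue damage on the target, applied on its Tick.
; Death clears AI targets, records the kill in game state, fires OnUnitDeath and detaches the controller.
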(event `self.ReceiveTick`
  (params (DeltaSeconds :type "Float (single-precision)"))
  (`self.ResetAttack` (`.AttackSpeed_10_8E5D2A574E278B3AEBACD687CBFB1DCF` (break `/Game/03_GameplayAssets/04_Data/01_Structs/ST_Unit_Stats` (`self.Stats`))))
  (`self.HandleBufferedDamageTaken`))

(event `self.ReceiveBeginPlay`
  (bind _asbp_auto_battler_ingame_controller (cast `/Game/03_GameplayAssets/01_Blueprints/01_Actors/01_Player/BP_AutoBattlerIngameController` (`GameplayStatics.GetPlayerController` 0)))
  (`/Game/03_GameplayAssets/01_Blueprints/01_Actors/01_Player/BP_AutoBattlerIngameController.RunOnServer_SpawnVFX` :`self` _asbp_auto_battler_ingame_controller :`Location` (`self.GetNavAgentLocation`) :`VFX` "/Game/05_VFX/UnitTeleportation/NS_UnitTeleportation.NS_UnitTeleportation")
  (add `self.OnUnitDeath` (`|CreateDelegate` :!event `OnDeathHandler`))
  (set `FloatingPawnMovement.MaxSpeed` (* (`.MovementSpeed_11_A5E599D64D7328C525321D961913D112` (break `/Game/03_GameplayAssets/04_Data/01_Structs/ST_Unit_Stats` (`self.Stats`))) (`self.MovementMultiplier`)) (`self.FloatingPawnMovement`)))

(event `OnDeathHandler` :!signature `self.OnUnitDeath`
  (params (RefToDeadUnit :type "/Game/03_GameplayAssets/01_Blueprints/01_Actors/02_Unit/BP_Unit Object Reference") (OwningPlayerSlotIndex :type Integer) (KillerPlayerSlotIndex :type Integer))
  (`self.PlayDeathSound`))

(event `TriggerAttackDamage`
  (params (Target :type "Self Object Reference") (Damage :type "Float (double-precision)") (AttackingPlayerSlotIndex :type Integer))
  (`KismetSystemLibrary.Delay` (`self.GeneralAttackDelay`))
  (`self.AddTakeDamage` Target Damage AttackingPlayerSlotIndex))

(event `PlayAttackSound`
  (params (Type :type Integer))
  (`AudioComponent.Play` (`self.AttackSFXCue`) 0.0))

(event `PlayDeathSound`
  (`AudioComponent.Play` (`self.SFX_Cue_Death`) 0.0))

(event `PlayIdleAnimation`
  (`SkeletalMeshComponent.PlayAnimation` (`self.SkeletalMesh`) (`self.IdleAnim`) false)
  (set `self.Walking` false))

(event `PlayDeathAnimation`
  (`SkeletalMeshComponent.PlayAnimation` (`self.SkeletalMesh`) (`self.DieAnim`) false)
  (set `self.Walking` false))

(event `PlayVictoryAnimation`
  (`SkeletalMeshComponent.PlayAnimation` (`self.SkeletalMesh`) (`self.VictoryAnim`) false)
  (set `self.Walking` false))

(event `PlayWalkAnimation`
  (`SkeletalMeshComponent.PlayAnimation` (`self.SkeletalMesh`) (`self.WalkAnim`) true)
  (set `self.Walking` true))

(event `PlayAttackAnimation`
  (`SkeletalMeshComponent.PlayAnimation` (`self.SkeletalMesh`) (`self.AttackAnim`) false)
  (set `self.Walking` false))

(event `PlayHitVFX`
  (`NiagaraFunctionLibrary.SpawnSystemAtLocation` "/Game/05_VFX/HitFeedBack/NS_HitFeedback.NS_HitFeedback" (`self.K2_GetActorLocation`) (struct) (10.0 10.0 10.0)))

(fn `AddTakeDamage`
  (params (Damage :type "Float (double-precision)") (AttackingPlayerSlotIndex :type Integer))
  (bind _isalive (`self.GetIsAlive`))
  (if _isalive
    (`KismetArrayLibrary.Array_Add` (`self.BufferedDamageTaken`) (make `/Game/03_GameplayAssets/04_Data/01_Structs/ST_AttackBuffer` null Damage AttackingPlayerSlotIndex))))

(fn `AttackTarget`
  (params (EnemyTarget :type "Self Object Reference"))
  (bind (_stats_dt_unitrowname _stats_cost _stats_upgradecost _stats_health _stats_movementspeed _stats_damage _stats_critchance _stats_critmultiplier _stats_range _stats_attackspeed _stats_maxhealth _stats_rank _stats_unittype) (break `/Game/03_GameplayAssets/04_Data/01_Structs/ST_Unit_Stats` (`self.Stats`)))
  (if (`KismetSystemLibrary.IsServer`)
    (if (stale _output_get)
      (bind _output_get (set `self.AttackReady` false))
      (set `self.lastAttack` (`GameplayStatics.GetTimeSeconds`))
      (bind _returnvalue (`self.CalculateAttackDamage`))
      (`|ExecutionSequence`
        (:`then_0`
          (`self.AddTakeDamage` EnemyTarget _returnvalue (`self.PlayerSlotIndex`)))
        (:`then_1`
          (`self.PlayAttackAnimation`)
          (`self.PlayAttackSound` _stats_unittype))))))

(fn `BufferedAttack`
  (bind _bufferedattacks (`self.BufferedAttacks`))
  (for _array_element _bufferedattacks
    (bind (_targetunit _damagetotake _attackingplayerslotid) (break `/Game/03_GameplayAssets/04_Data/01_Structs/ST_AttackBuffer` _array_element))
    (`/Engine/EditorBlueprintResources/StandardMacros.IsValid` _targetunit
      (:`Is Valid`
        (`self.AddTakeDamage` _targetunit _damagetotake _attackingplayerslotid))))
  (`KismetArrayLibrary.Array_Clear` _bufferedattacks))

(fn `CalculateAttackDamage`
  (returns (ReturnValue :type "Float (double-precision)"))
  (bind (_stats_dt_unitrowname _stats_cost _stats_upgradecost _stats_health _stats_movementspeed _stats_damage _stats_critchance _stats_critmultiplier) (break `/Game/03_GameplayAssets/04_Data/01_Structs/ST_Unit_Stats` (`self.Stats`)))
  (return (`KismetMathLibrary.SelectFloat` _stats_damage (* _stats_critmultiplier _stats_damage) (>= (`KismetMathLibrary.RandomFloatInRange` 0.0 100.0) _stats_critchance))))

(fn `FindSquare`
  (bind _returnvalue (`self.K2_GetActorLocation`))
  (bind _outhits (`KismetSystemLibrary.SphereTraceMulti` :`Start` _returnvalue :`End` (+ _returnvalue (0.0 0.0 1.0)) :`Radius` 20.0 :`TraceChannel` "TraceTypeQuery4" :`DrawDebugType` "ForOneFrame"))
  (for _array_element _outhits
    (if (== (`GameplayStatics.GetObjectClass` (`.HitActor` (`GameplayStatics.BreakHitResult` _array_element))) "/Game/03_GameplayAssets/01_Blueprints/01_Actors/03_Grid/BP_Square.BP_Square_C")
      (bind _asbp_square (cast `/Game/03_GameplayAssets/01_Blueprints/01_Actors/03_Grid/BP_Square` (`.HitActor` (`GameplayStatics.BreakHitResult` _array_element))))
      (`/Engine/EditorBlueprintResources/StandardMacros.IsValid` (`/Game/03_GameplayAssets/01_Blueprints/01_Actors/03_Grid/BP_Square.HostedUnit` _asbp_square)
        (:`Is Not Valid`
          (set `/Game/03_GameplayAssets/01_Blueprints/01_Actors/03_Grid/BP_Square.HostedUnit` self _asbp_square)
          (`self.K2_SetActorLocation` (`self.K2_GetActorLocation` _asbp_square))
          (break))))))

(fn `Fire Projectile`
  (locals (NewLocalVar :type "SkeletalMeshComponent Object Reference"))
  (bind _returnvalue (`|SpawnActorFromClass` "/Game/03_GameplayAssets/01_Blueprints/01_Actors/04_Projectile/BP_StraightShot.BP_StraightShot_C" (`KismetMathLibrary.MakeTransform` (`self.K2_GetActorLocation`) (`self.K2_GetActorRotation`)) "Undefined" "MultiplyWithRoot" null (0.0 0.0 0.0) (struct) null))
  (set `/Game/03_GameplayAssets/01_Blueprints/01_Actors/04_Projectile/BP_StraightShot.MaxRange` (* (`.Range_5_F1A0ADFA410819004523D4B1276AD43D` (break `/Game/03_GameplayAssets/04_Data/01_Structs/ST_Unit_Stats` (`self.Stats`))) 1.125) _returnvalue)
  (`self.SetLifeSpan` _returnvalue 1.5))

(fn `GetIsAlive`
  (returns (IsAlive :type Boolean))
  (return (> (`.Health_13_2DCE6A2B4475323F55B6BCBEB7E362CF` (break `/Game/03_GameplayAssets/04_Data/01_Structs/ST_Unit_Stats` (`self.Stats`))) 0.0)))

(fn `GetNextRank`
  (returns (UpgradedUnitStatsRowName :type Name) (HasUpgrade :type Boolean))
  (bind _returnvalue (`|GetDataTableRow` "/Game/03_GameplayAssets/04_Data/03_DataTables/DT_UnitStats.DT_UnitStats" (`self.UnitStatsRowName`))
    (:`then`
      (return (`.NextUpgradeUnitName_33_69C998184C5E71D08B059DB63C6BB127` (break `/Game/03_GameplayAssets/04_Data/01_Structs/ST_Unit_Stats` _returnvalue)) true))
    (:`RowNotFound`
      (return "None" false))))

(fn `HandleBufferedDamageTaken`
  (for _array_element (`self.BufferedDamageTaken`)
    (bind (_targetunit _damagetotake _attackingplayerslotid) (break `/Game/03_GameplayAssets/04_Data/01_Structs/ST_AttackBuffer` _array_element))
    (bind _iskilled (`self.TakeDamage` _damagetotake _attackingplayerslotid))
    (if _iskilled
      (break)))
  (`KismetArrayLibrary.Array_Clear` (`self.BufferedDamageTaken`)))

(fn `OnRep_CurrentHealth`
  (`self.Update Health Bar` (`self.CurrentHealth`) (`.MaxHealth_23_30E076974E2DDC5657E237922A9C3E06` (break `/Game/03_GameplayAssets/04_Data/01_Structs/ST_Unit_Stats` (`self.Stats`)))))

(fn `OnRep_UnitDataRow`
  (`self.SetupVisualComponents`))

(fn `OnRep_UnitLocation`
  (`self.K2_SetActorLocation` (`self.UnitLocation`))
  (`self.SetMeshRelativeZ` false))

(fn `OnRep_UnitStatsRowName`
  (bind _returnvalue (`|GetDataTableRow` "/Game/03_GameplayAssets/04_Data/03_DataTables/DT_UnitStats.DT_UnitStats" (`self.UnitStatsRowName`))
    (:`then`
      (bind _output_get (set `self.Stats` _returnvalue))
      (set `self.UnitDataRow` (make `DataTableRowHandle` "/Game/03_GameplayAssets/04_Data/03_DataTables/DT_Units.DT_Units" (`.DT_UnitRowName_41_F859CEF1428CA83B1C71E48546FD9C73` (break `/Game/03_GameplayAssets/04_Data/01_Structs/ST_Unit_Stats` _output_get))))
      (`self.RefreshVisualComponents`))))

(fn `RefreshVisualComponents`
  (locals (UnitMaterial :type "Material Object Reference"))
  (`self.SetupMeshVisuals`)
  (`self.SetupUnitHealthbar`)
  (`self.SetupUnitPlayerCircle`)
  (`self.SetupRankMarker`))

(fn `ResetAttack`
  (params (AttackPerSecond :type "Float (double-precision)"))
  (if (and (!= (`self.AttackReady`) true) (< (+ (`self.lastAttack`) (`KismetMathLibrary.SafeDivide` 1.0 AttackPerSecond)) (`GameplayStatics.GetTimeSeconds`)))
    (set `self.AttackReady` true)))

(fn `SetBattleUnit`
  (params (IsBattleUnit :type Boolean))
  (`self.SetReplicateMovement` IsBattleUnit))

(fn `SetDragState`
  (params (bEnabled :type Boolean))
  (`self.SetMeshRelativeZ` bEnabled))

(fn `SetFocused`
  (params (IsFocused :type Boolean))
  (bind _skeletalmesh (`self.SkeletalMesh`))
  (`PrimitiveComponent.SetRenderCustomDepth` _skeletalmesh IsFocused)
  (`PrimitiveComponent.SetCustomDepthStencilValue` _skeletalmesh 250))

(fn `SetHovered`
  (params (IsFocused :type Boolean))
  (bind _skeletalmesh (`self.SkeletalMesh`))
  (`PrimitiveComponent.SetRenderCustomDepth` _skeletalmesh IsFocused)
  (`PrimitiveComponent.SetCustomDepthStencilValue` _skeletalmesh 249))

(fn `SetMeshRelativeZ`
  (params (IsDragged :type Boolean))
  (locals (Offset :type "Float (double-precision)" :default 200.0))
  (if IsDragged
    (`SceneComponent.K2_SetRelativeLocation` (`self.SkeletalMesh`) (`KismetMathLibrary.MakeVector` 0.0 0.0 (`local.Offset`)) false false)
    (else
      (`SceneComponent.K2_SetRelativeLocation` (`self.SkeletalMesh`) (0.0 0.0 0.0) false false))))

(fn `SetStatsByDTRowName`
  (params (DT_UnitsStats_RowName :type Name))
  (set `self.UnitStatsRowName` DT_UnitsStats_RowName))

(fn `SetupMeshVisuals`
  (locals (UnitMaterial :type "Material Object Reference"))
  (bind _returnvalue (`|GetDataTableRow` "/Game/03_GameplayAssets/04_Data/03_DataTables/DT_Units.DT_Units" (`.RowName` (break `DataTableRowHandle` (`self.UnitDataRow`))))
    (:`then`
      (set `local.UnitMaterial` (`.Material_29_7CA25DB04F5A3F8AB580619D007D7943` (break `/Game/03_GameplayAssets/04_Data/01_Structs/ST_Units` _returnvalue)))
      (set `self.VictoryAnim` (`.VictoryAnim_38_1E173FE64433EC16D9B499AAAF97B22F` (break `/Game/03_GameplayAssets/04_Data/01_Structs/ST_Units` _returnvalue)))
      (set `self.AttackAnim` (`.AttackAnim_32_FF7F96BD463AACEFF18E8BA9E9A77A65` (break `/Game/03_GameplayAssets/04_Data/01_Structs/ST_Units` _returnvalue)))
      (set `self.IdleAnim` (`.IdleAnim_41_BCB5D3374A18B3D531278786A2CD3DF9` (break `/Game/03_GameplayAssets/04_Data/01_Structs/ST_Units` _returnvalue)))
      (set `self.DieAnim` (`.DieAnim_36_219BF17A44DB79708CB364A6924C672F` (break `/Game/03_GameplayAssets/04_Data/01_Structs/ST_Units` _returnvalue)))
      (set `self.WalkAnim` (`.WalkAnim_34_8346804946E7B4D3A52FDEBEA40DEAF8` (break `/Game/03_GameplayAssets/04_Data/01_Structs/ST_Units` _returnvalue)))
      (`SkeletalMeshComponent.SetSkeletalMeshAsset` (`self.SkeletalMesh`) (`.SekeltalMesh_11_032640014C81AFCA63D070BCA0DEE143` (break `/Game/03_GameplayAssets/04_Data/01_Structs/ST_Units` _returnvalue)))
      (bind _returnvalue_2 (`KismetMaterialLibrary.CreateDynamicMaterialInstance` (`local.UnitMaterial`)))
      (`PrimitiveComponent.SetMaterial` (`self.SkeletalMesh`) 0 _returnvalue_2)
      (`self.PlayIdleAnimation`))))

(fn `SetupRankMarker`
  (bind _aswbp_ui_unit_health_bar (cast `/Game/06_UI/01_Widgets/02_IngameWidgets/WBP_UI_UnitHealthBar` (`WidgetComponent.GetWidget` (`self.HealthBar`))))
  (`Image.SetBrushFromTexture` (`/Game/06_UI/01_Widgets/02_IngameWidgets/WBP_UI_UnitHealthBar.RankMarker` _aswbp_ui_unit_health_bar) (select `int` (- (`.Rank_27_9197347C41DB31474F6CA1AC08C0B1A9` (break `/Game/03_GameplayAssets/04_Data/01_Structs/ST_Unit_Stats` (`self.Stats`))) 1) :`0` "/Game/06_UI/01_Widgets/02_IngameWidgets/Rank1.Rank1" :`1` "/Game/06_UI/01_Widgets/02_IngameWidgets/Rank2.Rank2" :`2` "/Game/06_UI/01_Widgets/02_IngameWidgets/Rank3.Rank3" :!type "Texture2D Object Reference") false))

(fn `SetupUnitHealthbar`
  (bind _healthbar (`self.HealthBar`))
  (`SceneComponent.K2_SetRelativeLocation` (`self.HealthBar`) (* (`.BoxExtent` (`KismetSystemLibrary.GetComponentBounds` (`self.SkeletalMesh`))) (0.0 0.0 2.5)) false false)
  (bind _aswbp_ui_unit_health_bar (cast `/Game/06_UI/01_Widgets/02_IngameWidgets/WBP_UI_UnitHealthBar` (`WidgetComponent.GetWidget` _healthbar) :!label _label)
    (:`then`
      (`/Game/06_UI/01_Widgets/02_IngameWidgets/WBP_UI_UnitHealthBar.ScaleHealthbar` :`self` _aswbp_ui_unit_health_bar :`Actor` self))
    (:`CastFailed`
      (bind _returnvalue (`|CreateWidget` "/Game/06_UI/01_Widgets/02_IngameWidgets/WBP_UI_UnitHealthBar.WBP_UI_UnitHealthBar_C"))
      (`WidgetComponent.SetWidget` _healthbar _returnvalue)
      (goto _label))))

(fn `SetupUnitPlayerCircle`
  (bind _returnvalue (`PrimitiveComponent.CreateDynamicMaterialInstance` (`self.Sphere`) 0 "/Game/06_UI/05_Materials/StaticDisc_Instance.StaticDisc_Instance" "None"))
  (`MaterialInstanceDynamic.SetVectorParameterValue` _returnvalue "Color" (`/Game/03_GameplayAssets/01_Blueprints/90_MacroLibs/BPFL_GetGameSystem.GetPlayerSlotColorByIndex` (`self.PlayerSlotIndex`))))

(fn `SetupVisualComponents`
  (bind (_unitdatarow_datatable _unitdatarow_rowname) (break `DataTableRowHandle` (`self.UnitDataRow`)))
  (if (!= _unitdatarow_rowname "Default")
    (`|ExecutionSequence`
      (:`then_0`
        (`self.SetupMeshVisuals`))
      (:`then_1`
        (if (not (`self.IsInitialized`))
          (bind _returnvalue (`|GetDataTableRow` "/Game/03_GameplayAssets/04_Data/03_DataTables/DT_UnitStats.DT_UnitStats" _unitdatarow_rowname)
            (:`then`
              (set `self.Stats` _returnvalue)
              (`AudioParameterControllerInterface.SetIntParameter` (`self.AttackSFXCue`) "UnitType" (`.UnitType_30_84C92B224289F72A54AD749C00AB7E61` (break `/Game/03_GameplayAssets/04_Data/01_Structs/ST_Unit_Stats` _returnvalue)))
              (set `self.IsInitialized` true))))
        (`self.SetupUnitHealthbar`)
        (`self.SetupUnitPlayerCircle`)
        (`self.SetupRankMarker`)))))

(fn `TakeDamage`
  (params (Damage :type "Float (double-precision)") (PlayerSlotIndex :type Integer))
  (returns (IsKilled :type Boolean))
  (locals (SlotIndex :type Integer))
  (bind _healthbar (`self.HealthBar`))
  (bind _playerslotindex (`self.PlayerSlotIndex`))
  (bind _stats (`self.Stats`))
  (bind ((`UpgradeCost_44_F1F62F044C514F5CD8C661ABE38E2ECD` _upgradecost) (`Health_13_2DCE6A2B4475323F55B6BCBEB7E362CF` _health) (`MaxHealth_23_30E076974E2DDC5657E237922A9C3E06` _maxhealth)) (break `/Game/03_GameplayAssets/04_Data/01_Structs/ST_Unit_Stats` _stats))
  (bind _returnvalue (- _health Damage))
  ;[1 1 1] Reduce Health, by damage taken
  (if (> _health 0.0)
    (bind _structout (setmembers `/Game/03_GameplayAssets/04_Data/01_Structs/ST_Unit_Stats` :`StructRef` _stats :`Health` _returnvalue))
    (set `self.Stats` _structout)
    ;[1 1 1] Check if still alive
    (if (> _returnvalue 0.0)
      ;[1 1 1] Update Health Bar
      (bind _output_get (set `self.CurrentHealth` _returnvalue))
      (`self.Update Health Bar` _output_get _maxhealth)
      (`self.PlayHitVFX`)
      (return false)
      (else
        ;[1 1 1] Handle Death
        (bind _outactors (`GameplayStatics.GetAllActorsOfClass` "/Game/03_GameplayAssets/05_AI/BP_Unit_AI_Controller.BP_Unit_AI_Controller_C"))
        (for _array_element _outactors
          ;;[0.8316 0.4788 0.5426] Notify all units to remove dead unit from target + target lists
          (`KismetArrayLibrary.Array_RemoveItem` (`/Game/03_GameplayAssets/05_AI/BP_Unit_AI_Controller.TargetList` _array_element) self)
          (bind _returnvalue_2 (`AIBlueprintHelperLibrary.GetBlackboard` _array_element))
          (if (== self (`BlackboardComponent.GetValueAsObject` _returnvalue_2 "Current Target"))
            (`BlackboardComponent.ClearValue` _returnvalue_2 "Current Target")))
        (`/Game/03_GameplayAssets/06_GameSystem/03_GameStates/BP_AMB_IngameState.Add Killed Unit` (`/Game/03_GameplayAssets/01_Blueprints/90_MacroLibs/BPFL_GetGameSystem.GetAMBIngameState`) PlayerSlotIndex (`.RowName` (break `DataTableRowHandle` (`self.UnitDataRow`))) _playerslotindex)
        (`self.OnUnitDeath` self _playerslotindex PlayerSlotIndex)
        (`/Engine/EditorBlueprintResources/StandardMacros.IsValid` _healthbar
          (:`Is Valid`
            (`SceneComponent.SetVisibility` _healthbar false false))
          (:`Is Not Valid`
            _))
        (`self.PlayDeathAnimation`)
        (`self.DetachFromControllerPendingDestroy`)
        (return true)))))

(fn `Update Health Bar`
  (params (CurrentHealth :type "Float (double-precision)") (MaxHealth :type "Float (double-precision)"))
  (bind _healthbar (`self.HealthBar`))
  (bind _returnvalue (`WidgetComponent.GetWidget` _healthbar))
  (`/Engine/EditorBlueprintResources/StandardMacros.IsValid` _healthbar
    (:`Is Valid`
      (`/Engine/EditorBlueprintResources/StandardMacros.IsValid` _returnvalue
        (:`Is Valid`
          (bind _aswbp_ui_unit_health_bar (cast `/Game/06_UI/01_Widgets/02_IngameWidgets/WBP_UI_UnitHealthBar` _returnvalue))
          (`/Engine/EditorBlueprintResources/StandardMacros.IsValid` _aswbp_ui_unit_health_bar
            (:`Is Valid`
              (bind _healthbar_2 (`/Game/06_UI/01_Widgets/02_IngameWidgets/WBP_UI_UnitHealthBar.HealthBar` _aswbp_ui_unit_health_bar))
              (`/Engine/EditorBlueprintResources/StandardMacros.IsValid` _healthbar_2
                (:`Is Valid`
                  (`ProgressBar.SetPercent` _healthbar_2 (`KismetMathLibrary.SafeDivide` CurrentHealth MaxHealth)))))))))))

(fn `UserConstructionScript`
  (`self.SetupVisualComponents`))