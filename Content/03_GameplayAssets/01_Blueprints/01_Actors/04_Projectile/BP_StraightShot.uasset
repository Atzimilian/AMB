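; BP_StraightShot is a projectile actor with a Niagara effect, NSRangeUnitAttack, that expires once it covers the distance to its target.
; BeginPlay records the start position and sets max range as the distance to TargetLocation minus the effect's bounding sphere radius.
; Tick destroys the actor when its traveled distance reaches that range, with no hit logic in these graphs.
; The construction script tints the effect's burst and mesh colors.
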(event `self.ReceiveBeginPlay`
  (bind _output_get (set `self.StartPosition` (`self.K2_GetActorLocation`)))
  (set `self.MaxRange` (- (`KismetMathLibrary.Vector_Distance` _output_get (`self.TargetLocation`)) (`.SphereRadius` (`KismetSystemLibrary.GetComponentBounds` (`self.NS_RangeUnitAttack`))))))

(event `self.ReceiveTick`
  (params (DeltaSeconds :type "Float (single-precision)"))
  (if (>= (`KismetMathLibrary.Vector_Distance` (`self.StartPosition`) (`self.K2_GetActorLocation`)) (`self.MaxRange`))
    (`self.K2_DestroyActor`)))

(fn `UserConstructionScript`
  (locals (NewLocalVar :type "LinearColor Structure"))
  (bind _ns_rangeunitattack (`self.NS_RangeUnitAttack`))
  (bind _in_value (`self.In Value`))
  (`NiagaraComponent.SetVariableLinearColor` _ns_rangeunitattack "BurstColor" _in_value)
  (`NiagaraComponent.SetVariableLinearColor` _ns_rangeunitattack "MeshColor" _in_value))