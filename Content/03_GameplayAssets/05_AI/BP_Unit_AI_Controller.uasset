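; AI controller for units that starts and stops their behavior on demand.
; StartAI runs the BT_AI_UnitBehavior behavior tree, while StopAI halts the brain component's logic; both print status text and set an active flag.
; While active, Tick draws a debug arrow from the controlled pawn to the blackboard's Current Target actor.
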(event `StartAI`
  (`self.RunBehaviorTree` "/Game/03_GameplayAssets/05_AI/BT_AI_UnitBehavior.BT_AI_UnitBehavior")
  (`KismetSystemLibrary.PrintText` (`|FormatText` "AI Runing on unit {name}" (`self.GetParentActor`)))
  (set `self.AIActive` true))

(event `StopAI`
  (bind _braincomponent (`self.BrainComponent`))
  (`/Engine/EditorBlueprintResources/StandardMacros.IsValid` _braincomponent
    (:`Is Valid`
      (`BrainComponent.StopLogic` _braincomponent "")
      (`KismetSystemLibrary.PrintText` (`|FormatText` "AI Stopped :  {name}" (`self.K2_GetPawn`)))
      (set `self.AIActive` false))))

(event `self.ReceiveTick`
  (params (DeltaSeconds :type "Float (single-precision)"))
  (if (`self.AIActive`)
    (bind _asactor (cast `Actor` (`BlackboardComponent.GetValueAsObject` (`AIBlueprintHelperLibrary.GetBlackboard` null) (`KismetStringLibrary.Conv_StringToName` "Current Target"))))
    (`KismetSystemLibrary.DrawDebugArrow` (`self.K2_GetActorLocation` (`self.K2_GetPawn`)) (`self.K2_GetActorLocation` _asactor) 10.0 (struct) 2.0 5.0)))

(fn `UserConstructionScript`)