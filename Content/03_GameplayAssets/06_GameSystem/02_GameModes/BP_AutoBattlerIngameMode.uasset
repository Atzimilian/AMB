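; Game mode for the auto-battler match that runs a looping sequence of game phase objects, built at BeginPlay from an ordered class list.
; Each phase cycles through preparation, active, depreparation and transition states, advanced by a one-second timer mirrored to the first player controller.
; Transitions skip one phase type when four or fewer players remain alive.
; It also maps players to spawn points by slot index from game instance data.
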(event `self.ReceiveBeginPlay`
  (`|ExecutionSequence`
    (:`then_0`
      (`self.InitAllGamePhases`)
      (bind _outactors (`GameplayStatics.GetAllActorsOfClass` "/Game/03_GameplayAssets/01_Blueprints/01_Actors/03_Grid/BP_BattleOneIsland.BP_BattleOneIsland_C"))
      (set `self.BattleIslands` _outactors))
    (:`then_1`
      (bind _returnvalue (`GameplayStatics.GetActorOfClass` "/Game/03_GameplayAssets/01_Blueprints/01_Actors/03_Grid/BP_BattleRoyaleIsland.BP_BattleRoyaleIsland_C"))
      (set `self.BattleRoyaleIsland` _returnvalue))
    (:`then_2`
      (`KismetSystemLibrary.Delay` 2.0)
      (`self.InitFirstGamePhase`))))

(event `StartGamePhaseTimer`
  (params (TotalSeconds :type "Float (double-precision)"))
  (`self.StopGamePhaseTimer`)
  (set `self.GamePhaseTimerMaxSeconds` TotalSeconds)
  (set `self.GamePhaseTimerElapsedSeconds` 0.0)
  (bind _asbp_auto_battler_ingame_controller (cast `/Game/03_GameplayAssets/01_Blueprints/01_Actors/01_Player/BP_AutoBattlerIngameController` (`GameplayStatics.GetPlayerController` 0)))
  (`/Game/03_GameplayAssets/01_Blueprints/01_Actors/01_Player/BP_AutoBattlerIngameController.ServerRPC_SetupGamePhaseTimer` _asbp_auto_battler_ingame_controller TotalSeconds)
  (bind _returnvalue (`KismetSystemLibrary.K2_SetTimer` null "GamePhaseTimer_Interval" 1.0 true))
  (set `self.GamePhaseTimerHandle` _returnvalue))

(event `StopGamePhaseTimer`
  (`KismetSystemLibrary.K2_ClearAndInvalidateTimerHandle` (`self.GamePhaseTimerHandle`)))

(fn `ActivateCurrentGamePhase`
  (bind _currentgamephase (`self.CurrentGamePhase`))
  (`self.BeforeGamePhaseActive` _currentgamephase)
  (`/Game/03_GameplayAssets/06_GameSystem/05_GamePhases/BP_Base_GamePhase.ActivePhase` _currentgamephase)
  (`self.AfterGamePhaseActive` _currentgamephase))

(fn `ChoosePlayerStart`
  (params (Player :type "Controller Object Reference"))
  (returns (ReturnValue :type "Actor Object Reference"))
  (`self.InitSpawnPoints`)
  (bind _asbp_auto_battler_ingame_controller (cast `/Game/03_GameplayAssets/01_Blueprints/01_Actors/01_Player/BP_AutoBattlerIngameController` (`local.Player`)))
  (bind _playername (`AdvancedSessionsLibrary.GetPlayerName` _asbp_auto_battler_ingame_controller))
  (bind _foundplayerdata (`/Game/03_GameplayAssets/06_GameSystem/01_GameInstances/BP_AMB_GameInstance.GetPlayerDataByID` (`/Game/03_GameplayAssets/01_Blueprints/90_MacroLibs/BPFL_GetGameSystem.GetAMBGameInstance`) (`KismetStringLibrary.Conv_StringToName` _playername)))
  (set `/Game/03_GameplayAssets/01_Blueprints/01_Actors/01_Player/BP_AutoBattlerIngameController.OwnPlayerData` _foundplayerdata _asbp_auto_battler_ingame_controller)
  (bind ((`PlayerIdentifier_7_255E16A24A4681884D78149D2C13D6F6` _playeridentifier) (`PlayerNetIndex_22_F1933E6840869E4E8DD7999D5C0C20F0` _playernetindex) (`PlayerSlotIndex_19_821D2B7B47D671A0AD0677A89D4D41D4` _playerslotindex)) (break `/Game/03_GameplayAssets/04_Data/01_Structs/ST_PlayerData` _foundplayerdata))
  (`KismetSystemLibrary.PrintString` (`KismetStringLibrary.Concat_StrStr` _playername " | " (`KismetStringLibrary.Conv_NameToString` _playeridentifier)) true true (struct :`R` 1.0 :`G` 0.806522 :`A` 1.0) 10.0)
  (return (`BlueprintMapLibrary.Map_Find` (`self.PlayerSpawnPoints`) _playerslotindex)))

(fn `DebugTransitionNextGamePhase`
  (locals (PrevGamePhase :type "/Game/03_GameplayAssets/06_GameSystem/05_GamePhases/BP_Base_GamePhase Object Reference"))
  (bind _currentgamephase (`self.CurrentGamePhase`))
  (bind _returnvalue (mod (+ (`self.CurrentGamePhaseIndex`) 1) (`KismetArrayLibrary.Array_Length` (`self.GamePhaseOrderClasses`))))
  (bind _output (`|GetArrayItem` (`self.GamePhaseOrder`) _returnvalue))
  (`self.BeforeGamePhaseTransition` _currentgamephase _output)
  (`self.DepreparateCurrentGamePhase`)
  (set `local.PrevGamePhase` _currentgamephase)
  (set `self.CurrentGamePhaseIndex` _returnvalue)
  (set `self.CurrentGamePhase` _output)
  (`self.PreparateCurrentGamePhase`)
  (`self.AfterGamePhaseTransition` _output (`local.PrevGamePhase`)))

(fn `DepreparateCurrentGamePhase`
  (bind _currentgamephase (`self.CurrentGamePhase`))
  (`self.BeforeGamePhaseDepreparation` _currentgamephase)
  (`/Game/03_GameplayAssets/06_GameSystem/05_GamePhases/BP_Base_GamePhase.DepreparatePhase` _currentgamephase)
  (`self.AfterGamePhaseDepreparation` _currentgamephase))

(fn `EnterNextStateCurrentGamePhase`
  (set `self.CurrentGamePhaseState` (cast `/Game/03_GameplayAssets/04_Data/02_Enums/E_GamePhase_States` (mod (+ (`self.CurrentGamePhaseState`) 1) (`KismetMathLibrary.Conv_IntToByte` (enumcount `/Game/03_GameplayAssets/04_Data/02_Enums/E_GamePhase_States`)))))
  (`KismetSystemLibrary.PrintText` (`|FormatText` "Phase: {Phase} | State: {State}" (`|GetEnumeratorNameAsString` (`/Game/03_GameplayAssets/06_GameSystem/05_GamePhases/BP_Base_GamePhase.GamePhaseType` (`self.CurrentGamePhase`))) (`|GetEnumeratorNameAsString` (`self.CurrentGamePhaseState`))) true true (struct :`R` 1.0 :`G` 0.48837 :`A` 1.0) 60.0 "GamePhaseState")
  (switch `/Game/03_GameplayAssets/04_Data/02_Enums/E_GamePhase_States` (`self.CurrentGamePhaseState`)
    (:`NewEnumerator0`
      (`self.PreparateCurrentGamePhase`))
    (:`NewEnumerator1`
      (`self.ActivateCurrentGamePhase`))
    (:`NewEnumerator2`
      (`self.DepreparateCurrentGamePhase`))
    (:`NewEnumerator3`
      (`self.TransitionToNextGamePhase`))))

(fn `GamePhaseTimer_Interval`
  (bind _gamephasetimerelapsedseconds (`self.GamePhaseTimerElapsedSeconds`))
  (bind _result (`/Engine/EditorBlueprintResources/StandardMacros.IncrementFloat` (`self.GamePhaseTimerElapsedSeconds`))
    (:`  `
      (`KismetSystemLibrary.PrintText` (`|FormatText` "PhaseStateTimer: {ESec} / {MSec}" _result (`self.GamePhaseTimerMaxSeconds`)) true true (struct :`R` 0.977733 :`G` 1.0 :`A` 1.0) 1.15 "GamePhaseTimerText")
      (bind _asbp_auto_battler_ingame_controller (cast `/Game/03_GameplayAssets/01_Blueprints/01_Actors/01_Player/BP_AutoBattlerIngameController` (`GameplayStatics.GetPlayerController` 0)))
      (`/Game/03_GameplayAssets/01_Blueprints/01_Actors/01_Player/BP_AutoBattlerIngameController.ServerRPC_UpdateGamePhaseTimer` _asbp_auto_battler_ingame_controller _gamephasetimerelapsedseconds)
      (if (>= _gamephasetimerelapsedseconds (`self.GamePhaseTimerMaxSeconds`))
        (`self.StopGamePhaseTimer`)
        (`self.EnterNextStateCurrentGamePhase`)))))

(fn `GetNextGamePhase`
  (returns (OutputPin :type "/Game/03_GameplayAssets/06_GameSystem/05_GamePhases/BP_Base_GamePhase Object Reference") (ReturnValue :type Integer))
  (locals (NewGamePhaseIndex :type Integer) (NewGamePhase :type "/Game/03_GameplayAssets/06_GameSystem/05_GamePhases/BP_Base_GamePhase Object Reference"))
  (bind _gamephaseorder (`self.GamePhaseOrder`))
  (bind _gamephaseorder_2 (`self.GamePhaseOrder`))
  (bind _output_get (set `local.NewGamePhaseIndex` (mod (+ (`self.CurrentGamePhaseIndex`) 1) (`KismetArrayLibrary.Array_Length` _gamephaseorder))))
  (bind _output (`|GetArrayItem` _gamephaseorder _output_get))
  (set `local.NewGamePhase` _output)
  (if (and (<= (`/Game/03_GameplayAssets/06_GameSystem/03_GameStates/BP_AMB_IngameState.GetCountAlivePlayerSlotindices` (`/Game/03_GameplayAssets/01_Blueprints/90_MacroLibs/BPFL_GetGameSystem.GetAMBIngameState`)) 4) (`|EnumEquality` (`/Game/03_GameplayAssets/06_GameSystem/05_GamePhases/BP_Base_GamePhase.GamePhaseType` _output) "NewEnumerator1"))
    (bind _output_get_2 (set `local.NewGamePhaseIndex` (mod (+ (`local.NewGamePhaseIndex`) 1) (`KismetArrayLibrary.Array_Length` _gamephaseorder_2))))
    (set `local.NewGamePhase` (`|GetArrayItem` _gamephaseorder_2 _output_get_2)))
  (return (`local.NewGamePhase`) (`local.NewGamePhaseIndex`)))

(fn `InitAllGamePhases`
  (for _array_element (`self.GamePhaseOrderClasses`)
    (bind _returnvalue (`|GenericCreateObject` _array_element))
    (`KismetArrayLibrary.Array_Add` (`self.GamePhaseOrder`) _returnvalue)
    (`/Game/03_GameplayAssets/06_GameSystem/05_GamePhases/BP_Base_GamePhase.InitGamePhase` _returnvalue self (`/Game/03_GameplayAssets/01_Blueprints/90_MacroLibs/BPFL_GetGameSystem.GetAMBGameInstance`) (`/Game/03_GameplayAssets/01_Blueprints/90_MacroLibs/BPFL_GetGameSystem.GetAMBIngameState`))
    (set `self.CurrentGamePhase` (`|GetArrayItem` (`self.GamePhaseOrder`)))
    (set `self.CurrentGamePhaseIndex` 0)))

(fn `InitFirstGamePhase`
  (`/Game/03_GameplayAssets/06_GameSystem/05_GamePhases/BP_Base_GamePhase.PreparatePhase` (`self.CurrentGamePhase`))
  (`KismetSystemLibrary.PrintText` (`|FormatText` "Phase: {Phase} | State: {State}" (`|GetEnumeratorNameAsString` (`/Game/03_GameplayAssets/06_GameSystem/05_GamePhases/BP_Base_GamePhase.GamePhaseType` (`self.CurrentGamePhase`))) (`|GetEnumeratorNameAsString` (`self.CurrentGamePhaseState`))) true true (struct :`R` 1.0 :`G` 0.48837 :`A` 1.0) 60.0 "GamePhaseState"))

(fn `InitSpawnPoints`
  (if (== (`BlueprintMapLibrary.Map_Length` (`self.PlayerSpawnPoints`)) 0)
    (bind _outactors (`GameplayStatics.GetAllActorsOfClass` "/Game/03_GameplayAssets/01_Blueprints/01_Actors/01_Player/BP_AMB_PlayerStart.BP_AMB_PlayerStart_C"))
    (for _array_element _outactors
      (`BlueprintMapLibrary.Map_Add` (`self.PlayerSpawnPoints`) (`/Game/03_GameplayAssets/01_Blueprints/01_Actors/01_Player/BP_AMB_PlayerStart.GetPlayerIndex` _array_element) _array_element))))

(fn `PreparateCurrentGamePhase`
  (bind _currentgamephase (`self.CurrentGamePhase`))
  (`self.BeforeGamePhasePreperation` _currentgamephase)
  (`/Game/03_GameplayAssets/06_GameSystem/05_GamePhases/BP_Base_GamePhase.PreparatePhase` _currentgamephase)
  (`self.AfterGamePhasePreparation` _currentgamephase))

(fn `TransitionToNextGamePhase`
  (locals (PrevGamePhase :type "/Game/03_GameplayAssets/06_GameSystem/05_GamePhases/BP_Base_GamePhase Object Reference"))
  (bind _currentgamephase (`self.CurrentGamePhase`))
  (bind (_outputpin _returnvalue) (`self.GetNextGamePhase`))
  (`self.BeforeGamePhaseTransition` _currentgamephase _outputpin)
  (bind _output_get (set `local.PrevGamePhase` _currentgamephase))
  (`/Game/03_GameplayAssets/06_GameSystem/05_GamePhases/BP_Base_GamePhase.TransitionNextPhase` _output_get)
  (bind _output_get_2 (set `self.CurrentGamePhaseIndex` _returnvalue))
  (bind _output (`|GetArrayItem` (`self.GamePhaseOrder`) _output_get_2))
  (set `self.CurrentGamePhase` _output)
  (`self.AfterGamePhaseTransition` _output (`local.PrevGamePhase`))
  (`self.EnterNextStateCurrentGamePhase`))

(fn `UserConstructionScript`
  (`parent.UserConstructionScript`))