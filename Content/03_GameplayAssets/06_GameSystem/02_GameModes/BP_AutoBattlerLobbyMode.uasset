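; Lobby game mode for the auto battler that tracks connected players and their ready states, then server-travels to the in-game map on BeginMatch.
; Login and logout update the ConnectedPlayers struct array, and ready toggles flip the entry matching the player ID.
; Each change is forwarded through player controller 0, cast to the outgame controller, which receives the updated player data and whether all players are ready.
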(event `self.K2_PostLogin`
  (params (NewPlayer :type "PlayerController Object Reference"))
  ;[1 1 1] Player Dis-/Connects from/to our Session
  (`self.AddPlayerData` (`self.ExtractPlayerData` NewPlayer))
  (bind _asbp_auto_battler_outgame_controller (cast `/Game/03_GameplayAssets/01_Blueprints/01_Actors/01_Player/BP_AutoBattlerOutgameController` (`GameplayStatics.GetPlayerController` 0) :!label _label))
  (`/Game/03_GameplayAssets/01_Blueprints/01_Actors/01_Player/BP_AutoBattlerOutgameController.ServerRPC_ConnectedPlayersChanged` _asbp_auto_battler_outgame_controller (`self.ConnectedPlayers`))
  (bind _out_areallplayersready (`self.CheckAllPlayerReady`))
  (`/Game/03_GameplayAssets/01_Blueprints/01_Actors/01_Player/BP_AutoBattlerOutgameController.OnAllPlayersReadyState` _asbp_auto_battler_outgame_controller _out_areallplayersready))

(event `self.K2_OnLogout`
  (params (ExitingController :type "Controller Object Reference"))
  ;[1 1 1] Player Dis-/Connects from/to our Session
  (bind _asplayer_controller (cast `PlayerController` ExitingController))
  (`self.RemovePlayerData` (`self.ExtractPlayerData` _asplayer_controller))
  (goto _label))

(event `OnPlayerReadyStateChange`
  (params (PlayerDataID :type Name))
  ;[1 1 1] Player Toggles Ready State
  (`self.UpdatePlayerReadyState` PlayerDataID)
  (bind _asbp_auto_battler_outgame_controller (cast `/Game/03_GameplayAssets/01_Blueprints/01_Actors/01_Player/BP_AutoBattlerOutgameController` (`GameplayStatics.GetPlayerController` 0)))
  (bind _foundplayerdata (`self.GetPlayerDataByID` PlayerDataID))
  (`|ExecutionSequence`
    (:`then_0`
      (`/Game/03_GameplayAssets/01_Blueprints/01_Actors/01_Player/BP_AutoBattlerOutgameController.ServerRPC_UpdatePlayerReadyState` _asbp_auto_battler_outgame_controller _foundplayerdata))
    (:`then_1`
      (bind _out_areallplayersready (`self.CheckAllPlayerReady`))
      (`/Game/03_GameplayAssets/01_Blueprints/01_Actors/01_Player/BP_AutoBattlerOutgameController.OnAllPlayersReadyState` _asbp_auto_battler_outgame_controller _out_areallplayersready))))

(event `BeginMatch`
  (`AdvancedSessionsLibrary.ServerTravel` "SC_IngameMap"))

(fn `AddPlayerData`
  (params (PlayerData :type "/Game/03_GameplayAssets/04_Data/01_Structs/ST_PlayerData Structure"))
  (locals (isPlayerIDPresent :type Boolean))
  (`KismetArrayLibrary.Array_AddUnique` (`self.ConnectedPlayers`) PlayerData))

(fn `CheckAllPlayerReady`
  (returns (`Out AreAllPlayersReady` :type Boolean))
  (locals (AreAllPlayersReady :type Boolean))
  (set `local.AreAllPlayersReady` true)
  (for _array_element (`self.ConnectedPlayers`)
    (if (not (`.IsPlayerReady_16_4F0889D44E8145EC0D68BEA56D14DE0D` (break `/Game/03_GameplayAssets/04_Data/01_Structs/ST_PlayerData` _array_element)))
      (set `local.AreAllPlayersReady` false)
      (break)))
  (return (`local.AreAllPlayersReady`)))

(fn `GetPlayerDataByID`
  (params (PlayerDataID :type Name))
  (returns (FoundPlayerData :type "/Game/03_GameplayAssets/04_Data/01_Structs/ST_PlayerData Structure") (PlayerDataIndex :type Integer))
  (locals (PlayerData :type "/Game/03_GameplayAssets/04_Data/01_Structs/ST_PlayerData Structure") (PlayerDataIndexNumber :type Integer))
  (for (_array_element _array_index) (`self.ConnectedPlayers`)
    (if (== (`.PlayerIdentifier_7_255E16A24A4681884D78149D2C13D6F6` (break `/Game/03_GameplayAssets/04_Data/01_Structs/ST_PlayerData` _array_element)) PlayerDataID)
      (set `local.PlayerData` (`|GetArrayItem` (`self.ConnectedPlayers`) _array_index))
      (set `local.PlayerDataIndexNumber` _array_index)
      (break)))
  (return (`local.PlayerData`) (`local.PlayerDataIndexNumber`)))

(fn `GetPlayerDataByPC`
  (params (PlayerController :type "/Game/03_GameplayAssets/01_Blueprints/01_Actors/01_Player/BP_AutoBattlerPlayerController Object Reference"))
  (returns (FoundPlayerData :type "/Game/03_GameplayAssets/04_Data/01_Structs/ST_PlayerData Structure"))
  (locals (PlayerData :type "/Game/03_GameplayAssets/04_Data/01_Structs/ST_PlayerData Structure"))
  (for (_array_element _array_index) (`self.ConnectedPlayers`)
    (if (== (`.PC_Reference_14_E95BDABC43F5965C285E458338186E42` (break `/Game/03_GameplayAssets/04_Data/01_Structs/ST_PlayerData` _array_element)) PlayerController)
      (set `local.PlayerData` (`|GetArrayItem` (`self.ConnectedPlayers`) _array_index))
      (break)))
  (return (`local.PlayerData`)))

(fn `RemovePlayerData`
  (params (RemovingPlayerData :type "/Game/03_GameplayAssets/04_Data/01_Structs/ST_PlayerData Structure (by ref)"))
  (for (_array_element _array_index) (`self.ConnectedPlayers`)
    (if (== (`.PlayerIdentifier_7_255E16A24A4681884D78149D2C13D6F6` (break `/Game/03_GameplayAssets/04_Data/01_Structs/ST_PlayerData` _array_element)) RemovingPlayerData_PlayerIdentifier_7_255E16A24A4681884D78149D2C13D6F6)
      (`KismetArrayLibrary.Array_Remove` (`self.ConnectedPlayers`) _array_index)
      (break))))

(fn `UpdatePlayerReadyState`
  (params (PlayerDataID :type Name))
  (bind (_foundplayerdata _playerdataindex) (`self.GetPlayerDataByID` PlayerDataID))
  (bind (_playeridentifier _playername _pc_reference _isplayerready) (break `/Game/03_GameplayAssets/04_Data/01_Structs/ST_PlayerData` _foundplayerdata))
  (`/Engine/EditorBlueprintResources/StandardMacros.IsValid` _pc_reference
    (:`Is Valid`
      (bind _structout (setmembers `/Game/03_GameplayAssets/04_Data/01_Structs/ST_PlayerData` :`StructRef` _foundplayerdata :`IsPlayerReady` (not _isplayerready)))
      (`KismetArrayLibrary.Array_Set` (`self.ConnectedPlayers`) _playerdataindex _structout))))

(fn `UserConstructionScript`
  (`parent.UserConstructionScript`))