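; Game instance that hosts listen-server sessions and holds player lobby data and music across level changes.
; Host creates an Advanced Sessions session with a random name, then opens the level.
; Player slots and ready states live in SessionPlayerData, copied to IngamePlayerData at match start, though GetPlayerData always returns the session array.
; First music playback applies saved volumes through sound-mix class overrides, creating the save if absent.
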(event `self.ReceiveInit`
  ;[1 0.3137 0] Initialize ViewModel for connected Players [OBSOLETE]
)

(event `Host`
  (params (PlayerController :type "PlayerController Object Reference") (Level :type "World Soft Object Reference"))
  ;[1 1 1] Host Server /Create Session
  (bind _output_get (set `self.SessionName` (`KismetStringLibrary.Concat_StrStr` "GA_" (`KismetStringLibrary.Conv_IntToString` (`KismetMathLibrary.RandomIntegerInRange` 0 10)))))
  (`CreateSessionCallbackProxyAdvanced.CreateAdvancedSession` (`|MakeArray` (`AdvancedSessionsLibrary.MakeLiteralSessionPropertyString` "ServerName" _output_get) (`AdvancedSessionsLibrary.MakeLiteralSessionPropertyString` "GameIdentifier" "GA_SB_2024")) PlayerController (`self.MaxConnections`)
    (:`OnSuccess`
      (`GameplayStatics.OpenLevelBySoftObjectPtr` Level true "Listen"))))

(event `OnMatchStart`
  ;[1 1 1] Some Data needs to be secured on Scene Transition
  (set `self.IsMatchRunning` true)
  (`self.PrepareDataForMatchStart`))

(event `ResetLobbyMatchData`
  ;[1 1 1] When returning to Main Menu
  (set `self.IsMatchRunning` false)
  (`KismetArrayLibrary.Array_Clear` (`self.SessionPlayerData`))
  (`KismetArrayLibrary.Array_Clear` (`self.IngamePlayerData`)))

(event `Play Music`
  (params (Sound :type "SoundBase Object Reference"))
  (bind _music (`self.Music`))
  ;[1 1 1] Plays Music, continues across levels
  (`/Engine/EditorBlueprintResources/StandardMacros.IsValid` _music
    (:`Is Valid`
      (`AudioComponent.AdjustVolume` _music 2.0 1.0 "Linear")
      (`AudioComponent.FadeIn` _music 2.0 1.0 0.0 "Linear"))
    (:`Is Not Valid`
      (`GameplayStatics.SetBaseSoundMix` "/Game/07_Audio/02_Mixers/Mix_Global.Mix_Global")
      (`self.LoadAudioData`)
      (bind _returnvalue (`GameplayStatics.SpawnSound2D` Sound 1.0 1.0 0.0 null true))
      (set `self.Music` _returnvalue))))

(fn `AddPlayerData`
  (params (PlayerData :type "/Game/03_GameplayAssets/04_Data/01_Structs/ST_PlayerData Structure"))
  (locals (isPlayerIDPresent :type Boolean))
  (bind _out_emptyslotindex (`self.GetNextEmptySlot`))
  (bind _structout (setmembers `/Game/03_GameplayAssets/04_Data/01_Structs/ST_PlayerData` :`StructRef` PlayerData :`PlayerSlotIndex` _out_emptyslotindex))
  (`KismetArrayLibrary.Array_Add` (`self.SessionPlayerData`) _structout))

(fn `CheckAllPlayerReady`
  (returns (`Out AreAllPlayersReady` :type Boolean))
  (locals (AreAllPlayersReady :type Boolean))
  (set `local.AreAllPlayersReady` true)
  (for _array_element (`self.SessionPlayerData`)
    (if (not (`.IsPlayerReady_16_4F0889D44E8145EC0D68BEA56D14DE0D` (break `/Game/03_GameplayAssets/04_Data/01_Structs/ST_PlayerData` _array_element)))
      (set `local.AreAllPlayersReady` false)
      (break)))
  (return (`local.AreAllPlayersReady`)))

(fn `GetDataBySlotIndex`
  (params (PlayerDataSlotIndex :type Integer) (PlayerData :type "Array of /Game/03_GameplayAssets/04_Data/01_Structs/ST_PlayerData Structure"))
  (returns (FoundPlayerData :type "/Game/03_GameplayAssets/04_Data/01_Structs/ST_PlayerData Structure") (PlayerDataArrayIndex :type Integer) (`Result Found` :type Boolean))
  (locals (ArrayIndex :type Integer) (NewLocalVar :type "/Game/03_GameplayAssets/04_Data/01_Structs/ST_PlayerData Structure"))
  (bind _arrayindex (`local.ArrayIndex`))
  (bind _returnvalue (!= _arrayindex -1))
  (set `local.ArrayIndex` -1)
  (for (_array_element _array_index) PlayerData
    (if (== (`.PlayerSlotIndex_19_821D2B7B47D671A0AD0677A89D4D41D4` (break `/Game/03_GameplayAssets/04_Data/01_Structs/ST_PlayerData` _array_element)) PlayerDataSlotIndex)
      (set `local.ArrayIndex` _array_index)
      (break)))
  (if _returnvalue
    (return (`|GetArrayItem` PlayerData _arrayindex) _arrayindex _returnvalue)
    (else
      (return (struct) _arrayindex _returnvalue))))

(fn `GetNextEmptySlot`
  (returns (`Out EmptySlotIndex` :type Integer))
  (locals (EmptySlotIndex :type Integer))
  (for _index (range (`self.MaxConnections`))
    (bind (_foundplayerdata _playerdataarrayindex _result_found) (`self.GetDataBySlotIndex` _index (`self.SessionPlayerData`)))
    (if (not _result_found)
      (set `local.EmptySlotIndex` _index)
      (break)))
  (return (`local.EmptySlotIndex`)))

(fn `GetPlayerData`
  (returns (ReturnValue :type "Array of /Game/03_GameplayAssets/04_Data/01_Structs/ST_PlayerData Structure"))
  (bind _sessionplayerdata (`self.SessionPlayerData`))
  (return (select `bool` (`self.IsMatchRunning`) :`false` _sessionplayerdata :`true` _sessionplayerdata)))

(fn `GetPlayerDataByID`
  (params (PlayerDataID :type Name))
  (returns (FoundPlayerData :type "/Game/03_GameplayAssets/04_Data/01_Structs/ST_PlayerData Structure") (PlayerDataArrayIndex :type Integer) (`Result Found` :type Boolean))
  (locals (PlayerData :type "/Game/03_GameplayAssets/04_Data/01_Structs/ST_PlayerData Structure") (ArrayIndex :type Integer :default -1))
  (bind _arrayindex (`local.ArrayIndex`))
  (bind _returnvalue (!= _arrayindex -1))
  (set `local.ArrayIndex` -1)
  (for (_array_element _array_index) (`self.GetPlayerData`)
    (if (== (`.PlayerIdentifier_7_255E16A24A4681884D78149D2C13D6F6` (break `/Game/03_GameplayAssets/04_Data/01_Structs/ST_PlayerData` _array_element)) PlayerDataID)
      (set `local.ArrayIndex` _array_index)
      (break)))
  (if _returnvalue
    (return (`|GetArrayItem` (`self.GetPlayerData`) _arrayindex) _arrayindex _returnvalue)
    (else
      (return (struct) _arrayindex _returnvalue))))

(fn `GetPlayerDataByPC`
  (params (PlayerDataPC :type "/Game/03_GameplayAssets/01_Blueprints/01_Actors/01_Player/BP_AutoBattlerPlayerController Object Reference"))
  (returns (FoundPlayerData :type "/Game/03_GameplayAssets/04_Data/01_Structs/ST_PlayerData Structure") (PlayerDataArrayIndex :type Integer) (`Result Found` :type Boolean))
  (locals (PlayerData :type "/Game/03_GameplayAssets/04_Data/01_Structs/ST_PlayerData Structure") (ArrayIndex :type Integer))
  (bind (_foundplayerdata _playerdataarrayindex _result_found) (`self.GetPlayerDataByID` (`KismetStringLibrary.Conv_StringToName` (`AdvancedSessionsLibrary.GetPlayerName` PlayerDataPC))))
  (return _foundplayerdata _playerdataarrayindex _result_found))

(fn `GetPlayerDataBySlotIndex`
  (params (PlayerDataSlotIndex :type Integer))
  (returns (FoundPlayerData :type "/Game/03_GameplayAssets/04_Data/01_Structs/ST_PlayerData Structure") (PlayerDataArrayIndex :type Integer) (`Result Found` :type Boolean))
  (locals (ArrayIndex :type Integer) (NewLocalVar :type "/Game/03_GameplayAssets/04_Data/01_Structs/ST_PlayerData Structure"))
  (bind _arrayindex (`local.ArrayIndex`))
  (bind _returnvalue (!= _arrayindex -1))
  (set `local.ArrayIndex` -1)
  (for (_array_element _array_index) (`self.GetPlayerData`)
    (if (== (`.PlayerSlotIndex_19_821D2B7B47D671A0AD0677A89D4D41D4` (break `/Game/03_GameplayAssets/04_Data/01_Structs/ST_PlayerData` _array_element)) PlayerDataSlotIndex)
      (set `local.ArrayIndex` _array_index)
      (break)))
  (if _returnvalue
    (return (`|GetArrayItem` (`self.GetPlayerData`) _arrayindex) _arrayindex _returnvalue)
    (else
      (return (struct) _arrayindex _returnvalue))))

(fn `InitializeAudioData`)

(fn `LoadAudioData`
  (returns (`AsAudio Settings Save` :type "/Game/07_Audio/AudioSettingsSave Object Reference"))
  (locals (Filename :type String :default "AudioSettings"))
  (bind _filename (`local.Filename`))
  (bind _returnvalue (`GameplayStatics.DoesSaveGameExist` _filename :!label _label))
  (if _returnvalue
    (bind _returnvalue_2 (`GameplayStatics.LoadGameFromSlot` _filename))
    (`/Engine/EditorBlueprintResources/StandardMacros.IsValid` _returnvalue_2
      (:`Is Valid`
        (bind _asaudio_settings_save (cast `/Game/07_Audio/AudioSettingsSave` _returnvalue_2))
        (bind _audiosettings (`/Game/07_Audio/AudioSettingsSave.AudioLoad` _asaudio_settings_save))
        (`|ExecutionSequence`
          (:`then_0`
            (`GameplayStatics.SetSoundMixClassOverride` "/Game/07_Audio/02_Mixers/Mix_Global.Mix_Global" "/Game/07_Audio/02_Mixers/SC_Main.SC_Main" (break `/Game/03_GameplayAssets/04_Data/01_Structs/Struct_AudioSettings` _audiosettings) 1.0 0.0))
          (:`then_1`
            (`GameplayStatics.SetSoundMixClassOverride` "/Game/07_Audio/02_Mixers/Mix_Global.Mix_Global" "/Game/07_Audio/02_Mixers/SC_Music.SC_Music" (`.MusicVolume_9_4C68DEB843650E1C4FFE2B971FC6DA20` (break `/Game/03_GameplayAssets/04_Data/01_Structs/Struct_AudioSettings` _audiosettings)) 1.0 0.0))
          (:`then_2`
            (`GameplayStatics.SetSoundMixClassOverride` "/Game/07_Audio/02_Mixers/Mix_Global.Mix_Global" "/Game/07_Audio/02_Mixers/SC_SFX_Effects.SC_SFX_Effects" (`.EffectsVolume_8_5FC54A1C4AE7344C118C1EAEB91E16BD` (break `/Game/03_GameplayAssets/04_Data/01_Structs/Struct_AudioSettings` _audiosettings)) 1.0 0.0))
          (:`then_3`
            (`GameplayStatics.SetSoundMixClassOverride` "/Game/07_Audio/02_Mixers/Mix_Global.Mix_Global" "/Game/07_Audio/02_Mixers/SC_SFX_Voice.SC_SFX_Voice" (`.UIVolume_15_E68E803B4AB11AFEC804F5A100C3374E` (break `/Game/03_GameplayAssets/04_Data/01_Structs/Struct_AudioSettings` _audiosettings)) 1.0 0.0))
          (:`then_4`
            (`GameplayStatics.SetSoundMixClassOverride` "/Game/07_Audio/02_Mixers/Mix_Global.Mix_Global" "/Game/07_Audio/02_Mixers/SC_SFX_Ambient.SC_SFX_Ambient" (`.AmbientVolume_14_3C5B01BD4F41561DC3D3B8B6408372D4` (break `/Game/03_GameplayAssets/04_Data/01_Structs/Struct_AudioSettings` _audiosettings)) 1.0 0.0))
          (:`then_5`
            (return _asaudio_settings_save)))))
    (else
      (bind _returnvalue_3 (`GameplayStatics.CreateSaveGameObject` "/Game/07_Audio/AudioSettingsSave.AudioSettingsSave_C"))
      (set `/Game/07_Audio/AudioSettingsSave.AudioSettings` (struct) _returnvalue_3)
      (`self.SaveAudioData` true _returnvalue_3)
      (goto _label))))

(fn `PrepareDataForMatchStart`
  (bind _sessionplayerdata (`self.SessionPlayerData`))
  (for (_ _array_index) _sessionplayerdata
    (`KismetArrayLibrary.Array_Add` (`self.IngamePlayerData`) (`|GetArrayItem` _sessionplayerdata _array_index))))

(fn `RemovePlayerData`
  (params (RemovingPlayerData :type "/Game/03_GameplayAssets/04_Data/01_Structs/ST_PlayerData Structure (by ref)"))
  (bind _removingplayerdata_playeridentifier (break `/Game/03_GameplayAssets/04_Data/01_Structs/ST_PlayerData` (`local.RemovingPlayerData`)))
  (for (_array_element _array_index) (`self.SessionPlayerData`)
    (if (== (`.PlayerIdentifier_7_255E16A24A4681884D78149D2C13D6F6` (break `/Game/03_GameplayAssets/04_Data/01_Structs/ST_PlayerData` _array_element)) _removingplayerdata_playeridentifier)
      (`KismetArrayLibrary.Array_Remove` (`self.SessionPlayerData`) _array_index)
      (break))))

(fn `SaveAudioData`
  (params (Overwrite :type Boolean) (Data :type "SaveGame Object Reference"))
  (locals (`File Name` :type String :default "AudioSettings"))
  (bind _file_name (`local.File Name`))
  (bind _returnvalue (`GameplayStatics.DoesSaveGameExist` _file_name))
  (if _returnvalue
    (if Overwrite
      (`GameplayStatics.SaveGameToSlot` Data _file_name :!label _label))
    (else
      (goto _label))))

(fn `SetPlayerDataBySlotIndex`
  (params (PlayerDataSlotIndex :type Integer) (UpdatedPlayerData :type "/Game/03_GameplayAssets/04_Data/01_Structs/ST_PlayerData Structure (by ref)"))
  (returns (`Result Found` :type Boolean) (ReturnValue :type "Array of /Game/03_GameplayAssets/04_Data/01_Structs/ST_PlayerData Structure"))
  (locals (ArrayIndex :type Integer) (NewLocalVar :type "/Game/03_GameplayAssets/04_Data/01_Structs/ST_PlayerData Structure"))
  (bind _returnvalue (`self.GetPlayerData`))
  (bind _arrayindex (`local.ArrayIndex`))
  (bind _returnvalue_2 (!= _arrayindex -1))
  (set `local.ArrayIndex` -1)
  (for (_array_element _array_index) _returnvalue
    (if (== (`.PlayerSlotIndex_19_821D2B7B47D671A0AD0677A89D4D41D4` (break `/Game/03_GameplayAssets/04_Data/01_Structs/ST_PlayerData` _array_element)) PlayerDataSlotIndex)
      (set `local.ArrayIndex` _array_index)
      (break)))
  (if _returnvalue_2
    (`KismetArrayLibrary.Array_Set` (`self.GetPlayerData`) _arrayindex UpdatedPlayerData)
    (return _returnvalue_2 _returnvalue)
    (else
      (return _returnvalue_2))))

(fn `SwitchPlayerSlotIndex`
  (params (PlayerDataPC :type "/Game/03_GameplayAssets/01_Blueprints/01_Actors/01_Player/BP_AutoBattlerPlayerController Object Reference") (NewPlayerSlotIndex :type Integer))
  (locals (TempPlayerData :type "/Game/03_GameplayAssets/04_Data/01_Structs/ST_PlayerData Structure"))
  (bind (_foundplayerdata _playerdataarrayindex) (`self.GetPlayerDataByPC` PlayerDataPC))
  (setmembers `/Game/03_GameplayAssets/04_Data/01_Structs/ST_PlayerData` :`StructRef` (`|GetArrayItem` (`self.SessionPlayerData`) _playerdataarrayindex) :`PlayerSlotIndex` NewPlayerSlotIndex))

(fn `UpdatePlayerReadyState`
  (params (PlayerSlotIndex :type "Integer (by ref)") (PlayerID :type Name))
  (bind (_foundplayerdata _playerdataarrayindex) (`self.GetPlayerDataByID` PlayerID))
  (bind _output (`|GetArrayItem` (`self.SessionPlayerData`) _playerdataarrayindex))
  (setmembers `/Game/03_GameplayAssets/04_Data/01_Structs/ST_PlayerData` :`StructRef` _output :`IsPlayerReady` (not (`.IsPlayerReady_16_4F0889D44E8145EC0D68BEA56D14DE0D` (break `/Game/03_GameplayAssets/04_Data/01_Structs/ST_PlayerData` _output)))))