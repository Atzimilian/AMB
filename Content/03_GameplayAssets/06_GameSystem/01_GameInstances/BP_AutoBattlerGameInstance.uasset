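; Game instance for the auto battler that hosts multiplayer games.
; Its Host event creates an Advanced Sessions session with a random number as the server name, then opens the given level as a listen server on success.
; An obsolete, disconnected block once registered a connected-players ViewModel in the global MVVM collection, leaving Init empty.
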(event `self.ReceiveInit`
  ;[1 0.3137 0] Initialize ViewModel for connected Players [OBSOLETE]
)

(event `Host`
  (params (PlayerController :type "PlayerController Object Reference") (Level :type "World Soft Object Reference"))
  ;[1 1 1] Host Server /Create Session
  (`CreateSessionCallbackProxyAdvanced.CreateAdvancedSession` (`|MakeArray` (`AdvancedSessionsLibrary.MakeLiteralSessionPropertyString` "ServerName" (`KismetStringLibrary.Conv_IntToString` (`KismetMathLibrary.RandomIntegerInRange` 0 100)))) PlayerController (`self.MaxConnections`)
    (:`OnSuccess`
      (`GameplayStatics.OpenLevelBySoftObjectPtr` Level true "Listen"))))