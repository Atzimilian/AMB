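; In-game Game State for the auto battler, holding match data: player stats, grid unit placements, kill tallies, ready count and deaths.
; The server seeds player data from the Game Instance, and slot index and grid coordinate lookups drive edits to it.
; Battle outcomes update health and kill points, then reach the player's controller by RPC.
; Dispatchers signal currency awards and building phase changes, while RepNotify on deaths opens death or win overlays.
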(event `self.ReceiveBeginPlay`
  (`parent.ReceiveBeginPlay`)
  (cast `/Game/03_GameplayAssets/01_Blueprints/01_Actors/01_Player/BP_AutoBattlerIngameController` (`GameplayStatics.GetPlayerController` 0)))

(event `RecieveOutcome`
  (params (Loss :type "/Game/03_GameplayAssets/04_Data/01_Structs/ST_BattleResult Structure"))
  ;[1 1 1] Display Battle Results - post battle
  (`self.UpdatePlayerMatchStats` Loss)
  (bind (_playercontroller _success) (`self.GetPlayerControllerBySlotIndex` (`.SlotID_26_92C8071B4C405CF822BF6F870D5CE8AE` (break `/Game/03_GameplayAssets/04_Data/01_Structs/ST_BattleResult` Loss))))
  (if _success
    (`/Game/03_GameplayAssets/01_Blueprints/01_Actors/01_Player/BP_AutoBattlerIngameController.OwningClientRPC_OnBattleOutcomeRecieve` _playercontroller Loss)))

(fn `Add Killed Unit`
  (params (KillerSlotIndex :type Integer) (KilledUnit :type Name) (OwnerSlotIndex :type Integer))
  (locals (`Array Index` :type Integer :default -1))
  (for (_array_element _array_index) (`self.KilledUnits`)
    (bind (_killerslotindex _killedunit _killedcount _ownerslotindex) (break `/Game/03_GameplayAssets/04_Data/01_Structs/ST_KilledUnits` _array_element))
    (if (and (== _killerslotindex KillerSlotIndex) (== _killedunit KilledUnit) (== _ownerslotindex OwnerSlotIndex))
      (bind _output_get (set `local.Array Index` _array_index))
      (bind _result (`/Engine/EditorBlueprintResources/StandardMacros.IncrementInt` _killedcount)
        (:`  `
          (break)))))
  (if (!= (`local.Array Index`) -1)
    (`KismetArrayLibrary.Array_Set` (`self.KilledUnits`) _output_get (make `/Game/03_GameplayAssets/04_Data/01_Structs/ST_KilledUnits` KillerSlotIndex KilledUnit _result OwnerSlotIndex))
    (else
      (`KismetArrayLibrary.Array_Append` (`self.KilledUnits`) (`|MakeArray` (make `/Game/03_GameplayAssets/04_Data/01_Structs/ST_KilledUnits` KillerSlotIndex KilledUnit 1 OwnerSlotIndex))))))

(fn `AddDeadPlayer`
  (params (SlotID :type Integer))
  (bind _playerdeaths (`self.PlayerDeaths`))
  (if (== (`KismetArrayLibrary.Array_Find` _playerdeaths SlotID) -1)
    (`KismetArrayLibrary.Array_Add` _playerdeaths SlotID)
    (set `self.PlayerDeaths` _playerdeaths)
    (bind _playercontroller (`self.GetPlayerControllerBySlotIndex` SlotID))
    (set `/Game/03_GameplayAssets/01_Blueprints/01_Actors/01_Player/BP_AutoBattlerIngameController.Dead` true _playercontroller)))

(fn `AddMatchReadyPlayer`
  (returns (AreAllPlayersMatchReady :type Boolean))
  (bind _result (`/Engine/EditorBlueprintResources/StandardMacros.IncrementInt` (`self.MatchReadyPlayers`))
    (:`  `
      (return (>= _result (`KismetArrayLibrary.Array_Length` (`self.IngamePlayerData`)))))))

(fn `AwardCurrency`
  (if (`KismetSystemLibrary.IsServer`)
    (`self.CurrencyAwarded`)))

(fn `BattleIslandFinished`)

(fn `GetCountAlivePlayerSlotindices`
  (returns (CountAlivePlayerSlotindices :type Integer))
  (return (`KismetArrayLibrary.Array_Length` (`self.AlivePlayerSlotIndices`))))

(fn `GetPlayerControllerBySlotIndex`
  (params (PlayerSlotIndex :type Integer))
  (returns (PlayerController :type "/Game/03_GameplayAssets/01_Blueprints/01_Actors/01_Player/BP_AutoBattlerIngameController Object Reference") (Success :type Boolean))
  (locals (FoundPlayerController :type "/Game/03_GameplayAssets/01_Blueprints/01_Actors/01_Player/BP_AutoBattlerIngameController Object Reference") (IsSuccess :type Boolean))
  (for _array_element (`self.PlayerArray`)
    (bind _asbp_auto_battler_ingame_controller (cast `/Game/03_GameplayAssets/01_Blueprints/01_Actors/01_Player/BP_AutoBattlerIngameController` (`PlayerState.GetPlayerController` _array_element)))
    (if (== (`.PlayerSlotIndex_19_821D2B7B47D671A0AD0677A89D4D41D4` (break `/Game/03_GameplayAssets/04_Data/01_Structs/ST_PlayerData` (`/Game/03_GameplayAssets/01_Blueprints/01_Actors/01_Player/BP_AutoBattlerIngameController.OwnPlayerData` _asbp_auto_battler_ingame_controller))) PlayerSlotIndex)
      (set `local.FoundPlayerController` _asbp_auto_battler_ingame_controller)
      (set `local.IsSuccess` true)
      (break)))
  (return (`local.FoundPlayerController`) (`local.IsSuccess`)))

(fn `GetPlayerDataBySlotIndex`
  (params (PlayerSlotIndex :type Integer))
  (returns (FoundPlayerData :type "/Game/03_GameplayAssets/04_Data/01_Structs/ST_PlayerData Structure") (PlayerDataArrayIndex :type Integer) (`Result Found` :type Boolean))
  (locals (ArrayIndex :type Integer))
  (bind _arrayindex (`local.ArrayIndex`))
  (bind _returnvalue (!= _arrayindex -1))
  (for (_array_element _array_index) (`self.IngamePlayerData`)
    (if (== (`.PlayerSlotIndex_19_821D2B7B47D671A0AD0677A89D4D41D4` (break `/Game/03_GameplayAssets/04_Data/01_Structs/ST_PlayerData` _array_element)) PlayerSlotIndex)
      (set `local.ArrayIndex` _array_index)
      (break)))
  (if _returnvalue
    (return (`|GetArrayItem` (`self.IngamePlayerData`) _arrayindex) _arrayindex _returnvalue)
    (else
      (return (struct) _arrayindex _returnvalue))))

(fn `GetPlayerUnitByGridCoord`
  (params (OwningPlayerSlotIndex :type Integer) (GridCoord :type "/Game/03_GameplayAssets/04_Data/01_Structs/ST_GridCoords Structure") (PlayerGridUnits :type "Array of /Game/03_GameplayAssets/04_Data/01_Structs/ST_PlayerUnit Structure"))
  (returns (FoundPlayerUnit :type "/Game/03_GameplayAssets/04_Data/01_Structs/ST_PlayerUnit Structure") (PlayerUnitArrayIndex :type Integer) (`Result Found` :type Boolean))
  (locals (ArrayIndex :type Integer))
  (bind (_xindex _yindex) (break `/Game/03_GameplayAssets/04_Data/01_Structs/ST_GridCoords` GridCoord))
  (bind _arrayindex (`local.ArrayIndex`))
  (bind _returnvalue (!= _arrayindex -1))
  (set `local.ArrayIndex` -1)
  (for (_array_element _array_index) PlayerGridUnits
    (bind (_owningplayerslotindex _gridx _gridy) (break `/Game/03_GameplayAssets/04_Data/01_Structs/ST_PlayerUnit` _array_element))
    (if (and (== _owningplayerslotindex OwningPlayerSlotIndex) (== _gridx _xindex) (== _gridy _yindex))
      (set `local.ArrayIndex` _array_index)
      (break)))
  (if _returnvalue
    (return (`|GetArrayItem` PlayerGridUnits _arrayindex) _arrayindex _returnvalue)
    (else
      (return (struct) _arrayindex _returnvalue))))

(fn `GetPlayerUnitsOfPlayerSlotIndex`
  (params (OwningPlayerSlotIndex :type Integer))
  (returns (OutPlayerOwningUnits :type "Array of /Game/03_GameplayAssets/04_Data/01_Structs/ST_PlayerUnit Structure"))
  (locals (PlayerOwningUnits :type "Array of /Game/03_GameplayAssets/04_Data/01_Structs/ST_PlayerUnit Structure"))
  (for _array_element (`self.PlayerUnits`)
    (if (== (`.OwningPlayerSlotIndex_12_8369573341323E2A295DAEA2ED3DA911` (break `/Game/03_GameplayAssets/04_Data/01_Structs/ST_PlayerUnit` _array_element)) OwningPlayerSlotIndex)
      (`KismetArrayLibrary.Array_Add` (`local.PlayerOwningUnits`) _array_element)))
  (return (`local.PlayerOwningUnits`)))

(fn `OnRep_IsPlayerBuildingEnabled`
  (if true
    (bind _asbp_auto_battler_ingame_controller (cast `/Game/03_GameplayAssets/01_Blueprints/01_Actors/01_Player/BP_AutoBattlerIngameController` (`GameplayStatics.GetPlayerController` 0)))
    (if (== (`KismetArrayLibrary.Array_Find` (`self.PlayerDeaths`) (`.PlayerSlotIndex_19_821D2B7B47D671A0AD0677A89D4D41D4` (break `/Game/03_GameplayAssets/04_Data/01_Structs/ST_PlayerData` (`/Game/03_GameplayAssets/01_Blueprints/01_Actors/01_Player/BP_AutoBattlerIngameController.OwnPlayerData` _asbp_auto_battler_ingame_controller)))) -1)
      (`self.OnPlayerBuildingEnabledChange` (`self.IsPlayerBuildingEnabled`)))))

(fn `OnRep_PlayerDeaths`
  (bind _playerdeaths (`self.PlayerDeaths`))
  (bind _returnvalue (`KismetArrayLibrary.Array_LastIndex` _playerdeaths))
  (bind _returnvalue_2 (- (`self.MatchReadyPlayers`) _returnvalue))
  (bind _asbp_auto_battler_ingame_controller (cast `/Game/03_GameplayAssets/01_Blueprints/01_Actors/01_Player/BP_AutoBattlerIngameController` (`GameplayStatics.GetPlayerController` 0)))
  (bind ((`PlayerSlotIndex_19_821D2B7B47D671A0AD0677A89D4D41D4` _playerslotindex)) (break `/Game/03_GameplayAssets/04_Data/01_Structs/ST_PlayerData` (`/Game/03_GameplayAssets/01_Blueprints/01_Actors/01_Player/BP_AutoBattlerIngameController.OwnPlayerData` _asbp_auto_battler_ingame_controller)))
  (if (== _playerslotindex (`|GetArrayItem` _playerdeaths _returnvalue))
    (bind _asbp_ingame_hud (cast `/Game/03_GameplayAssets/06_GameSystem/04_HUD/BP_IngameHUD` (`PlayerController.GetHUD` _asbp_auto_battler_ingame_controller)))
    (bind _returnvalue_3 (`/Game/06_UI/01_Widgets/01_BaseElements/WBP_MenuBase.PushToPopUp` (`/Game/03_GameplayAssets/06_GameSystem/04_HUD/BP_BaseHUD.WBPMenuStack` _asbp_ingame_hud) "/Game/06_UI/01_Widgets/06_GameHUDWidgets/WBP_Overlay_DeathScreen.WBP_Overlay_DeathScreen_C"))
    (bind _aswbp_overlay_death_screen (cast `/Game/06_UI/01_Widgets/06_GameHUDWidgets/WBP_Overlay_DeathScreen` _returnvalue_3))
    (`/Game/06_UI/01_Widgets/06_GameHUDWidgets/WBP_Overlay_DeathScreen.SetPlace` _aswbp_overlay_death_screen _returnvalue_2 (`self.MatchReadyPlayers`))
    (elif (and (== _returnvalue_2 2) (== (`KismetArrayLibrary.Array_Find` _playerdeaths _playerslotindex) -1))
      (bind _asbp_ingame_hud_2 (cast `/Game/03_GameplayAssets/06_GameSystem/04_HUD/BP_IngameHUD` (`PlayerController.GetHUD` _asbp_auto_battler_ingame_controller)))
      (`/Game/06_UI/01_Widgets/01_BaseElements/WBP_MenuBase.PushToPopUp` (`/Game/03_GameplayAssets/06_GameSystem/04_HUD/BP_BaseHUD.WBPMenuStack` _asbp_ingame_hud_2) "/Game/06_UI/01_Widgets/06_GameHUDWidgets/WBP_Overlay_WinScreen.WBP_Overlay_WinScreen_C"))))

(fn `RecieveBattleOneResult`
  (params (Result :type "/Game/03_GameplayAssets/04_Data/01_Structs/ST_BattleResult Structure (by ref)"))
  (`KismetArrayLibrary.Array_Add` (`self.BattleOneResults`) Result))

(fn `RemovePlayerUnitInGrid`
  (params (PlayerSlotIndex :type Integer) (GridCoord :type "/Game/03_GameplayAssets/04_Data/01_Structs/ST_GridCoords Structure"))
  (bind _playerunits (`self.PlayerUnits`))
  (bind (_foundplayerunit _playerunitarrayindex _result_found) (`self.GetPlayerUnitByGridCoord` PlayerSlotIndex GridCoord _playerunits))
  (if _result_found
    (`KismetArrayLibrary.Array_Remove` _playerunits _playerunitarrayindex)))

(fn `ResetKilledUnits`
  (`KismetArrayLibrary.Array_Clear` (`self.KilledUnits`)))

(fn `ResolveAlivePlayerSlotIndices`
  (returns (OutAlivePlayers :type "Array of Integer"))
  (`KismetArrayLibrary.Array_Clear` (`self.AlivePlayerSlotIndices`))
  (for _array_element (`self.IngamePlayerData`)
    (bind ((`PlayerSlotIndex_19_821D2B7B47D671A0AD0677A89D4D41D4` _playerslotindex) (`PlayerMatchStats_25_8CBF88AC4F0E129A8AF86D9EB811D0B8` _playermatchstats)) (break `/Game/03_GameplayAssets/04_Data/01_Structs/ST_PlayerData` _array_element))
    (if (> (`.Health_14_1C46CA4E40AC9850F252D289B69847ED` (break `/Game/03_GameplayAssets/04_Data/01_Structs/ST_MatchStats` _playermatchstats)) 0)
      (`KismetArrayLibrary.Array_Add` (`self.AlivePlayerSlotIndices`) _playerslotindex)))
  (return (`self.AlivePlayerSlotIndices`)))

(fn `SetIsPlayerBuildingEnabled`
  (params (IsPlayerBuildingEnabled :type Boolean))
  (bind _output_get (set `self.IsPlayerBuildingEnabled` IsPlayerBuildingEnabled))
  (if (`KismetSystemLibrary.IsServer`)
    (`self.OnPlayerBuildingEnabledChange` _output_get)))

(fn `SetPlayerDataBySlotIndex`
  (params (PlayerSlotIndex :type Integer) (UpdatedPlayerData :type "/Game/03_GameplayAssets/04_Data/01_Structs/ST_PlayerData Structure"))
  (returns (`Result Found` :type Boolean))
  (locals (ArrayIndex :type Integer))
  (bind _arrayindex (`local.ArrayIndex`))
  (bind _returnvalue (!= _arrayindex -1))
  (for (_array_element _array_index) (`self.IngamePlayerData`)
    (if (== (`.PlayerSlotIndex_19_821D2B7B47D671A0AD0677A89D4D41D4` (break `/Game/03_GameplayAssets/04_Data/01_Structs/ST_PlayerData` _array_element)) PlayerSlotIndex)
      (set `local.ArrayIndex` _array_index)
      (break)))
  (if _returnvalue
    (`KismetArrayLibrary.Array_Set` (`self.IngamePlayerData`) _arrayindex UpdatedPlayerData)
    (return _returnvalue)
    (else
      (return _returnvalue))))

(fn `SwapPlayerUnitsInGrid`
  (params (PlayerSlotIndex :type Integer) (UnitAGridCoord :type "/Game/03_GameplayAssets/04_Data/01_Structs/ST_GridCoords Structure") (UnitBGridCoord :type "/Game/03_GameplayAssets/04_Data/01_Structs/ST_GridCoords Structure"))
  (locals (UnitA :type "/Game/03_GameplayAssets/04_Data/01_Structs/ST_PlayerUnit Structure") (UnitB :type "/Game/03_GameplayAssets/04_Data/01_Structs/ST_PlayerUnit Structure"))
  (bind (_unitbgridcoord_xindex _unitbgridcoord_yindex) (break `/Game/03_GameplayAssets/04_Data/01_Structs/ST_GridCoords` (`local.UnitBGridCoord`)))
  (bind _playerunits (`self.PlayerUnits`))
  (bind (_unitagridcoord_xindex _unitagridcoord_yindex) (break `/Game/03_GameplayAssets/04_Data/01_Structs/ST_GridCoords` (`local.UnitAGridCoord`)))
  (`|ExecutionSequence`
    (:`then_0`
      (bind (_foundplayerunit _playerunitarrayindex) (`self.GetPlayerUnitByGridCoord` 0 UnitAGridCoord _playerunits))
      (set `local.UnitA` _foundplayerunit))
    (:`then_1`
      (bind (_foundplayerunit_2 _playerunitarrayindex_2) (`self.GetPlayerUnitByGridCoord` 0 UnitBGridCoord _playerunits))
      (set `local.UnitB` _foundplayerunit_2))
    (:`then_2`
      (bind _structout (setmembers `/Game/03_GameplayAssets/04_Data/01_Structs/ST_PlayerUnit` :`StructRef` (`local.UnitA`) :`GridX` _unitbgridcoord_xindex :`GridY` _unitbgridcoord_yindex))
      (`KismetArrayLibrary.Array_Set` (`self.PlayerUnits`) _playerunitarrayindex _structout)
      (bind _structout_2 (setmembers `/Game/03_GameplayAssets/04_Data/01_Structs/ST_PlayerUnit` :`StructRef` (`local.UnitB`) :`GridX` _unitagridcoord_xindex :`GridY` _unitagridcoord_yindex))
      (`KismetArrayLibrary.Array_Set` (`self.PlayerUnits`) _playerunitarrayindex_2 _structout_2))))

(fn `UpdatePlayerMatchStats`
  (params (MatchResults :type "/Game/03_GameplayAssets/04_Data/01_Structs/ST_BattleResult Structure"))
  (bind ((`KillScore_15_0652BE904981294D1B69E6A9E9BF2B9D` _killscore) (`LostHealth_19_780462124D662D5F6C746FB6538E365A` _losthealth) (`SlotID_26_92C8071B4C405CF822BF6F870D5CE8AE` _slotid)) (break `/Game/03_GameplayAssets/04_Data/01_Structs/ST_BattleResult` MatchResults))
  (bind (_foundplayerdata _playerdataarrayindex _result_found) (`self.GetPlayerDataBySlotIndex` _slotid))
  (if _result_found
    (bind ((`PC_Reference_14_E95BDABC43F5965C285E458338186E42` _pc_reference) (`PlayerMatchStats_25_8CBF88AC4F0E129A8AF86D9EB811D0B8` _playermatchstats)) (break `/Game/03_GameplayAssets/04_Data/01_Structs/ST_PlayerData` _foundplayerdata))
    (bind ((`KillPoints_15_1F6314D145CCCA4987567B8980C75890` _killpoints) (`Health_14_1C46CA4E40AC9850F252D289B69847ED` _health)) (break `/Game/03_GameplayAssets/04_Data/01_Structs/ST_MatchStats` _playermatchstats))
    (bind _structout (setmembers `/Game/03_GameplayAssets/04_Data/01_Structs/ST_MatchStats` :`StructRef` _playermatchstats :`KillPoints` (+ _killpoints _killscore) :`Health` (- _health _losthealth)))
    (bind _structout_2 (setmembers `/Game/03_GameplayAssets/04_Data/01_Structs/ST_PlayerData` :`StructRef` _foundplayerdata :`PlayerMatchStats` _structout))
    (`self.SetPlayerDataBySlotIndex` _slotid _structout_2)
    (bind _asbp_auto_battler_ingame_controller (cast `/Game/03_GameplayAssets/01_Blueprints/01_Actors/01_Player/BP_AutoBattlerIngameController` _pc_reference))
    (set `/Game/03_GameplayAssets/01_Blueprints/01_Actors/01_Player/BP_AutoBattlerIngameController.OwnPlayerData` _structout_2 _asbp_auto_battler_ingame_controller)
    (bind _asbp_auto_battler_ingame_controller_2 (cast `/Game/03_GameplayAssets/01_Blueprints/01_Actors/01_Player/BP_AutoBattlerIngameController` (`GameplayStatics.GetPlayerController` 0)))
    (`/Game/03_GameplayAssets/01_Blueprints/01_Actors/01_Player/BP_AutoBattlerIngameController.ServerRPC_NotifyUpdatedMatchStats` _asbp_auto_battler_ingame_controller_2 _structout_2)))

(fn `UpdatePlayerUnitInGrid`
  (params (OwningPlayerSlotIndex :type Integer) (OriginGridCoord :type "/Game/03_GameplayAssets/04_Data/01_Structs/ST_GridCoords Structure") (NewGridCoord :type "/Game/03_GameplayAssets/04_Data/01_Structs/ST_GridCoords Structure") (UnitTypeRowName :type Name) (UnitStats_RowName :type Name))
  (bind _playerunits (`self.PlayerUnits`))
  (bind (_newgridcoord_xindex _newgridcoord_yindex) (break `/Game/03_GameplayAssets/04_Data/01_Structs/ST_GridCoords` (`local.NewGridCoord`)))
  (bind (_newgridcoord_xindex_2 _newgridcoord_yindex_2) (break `/Game/03_GameplayAssets/04_Data/01_Structs/ST_GridCoords` (`local.NewGridCoord`)))
  (if (not (and (== OriginGridCoord_XIndex_2_AB621A1342F13200DFB3D5A823080C0A NewGridCoord_XIndex_2_AB621A1342F13200DFB3D5A823080C0A) (== OriginGridCoord_YIndex_4_0534BDCC457A222D875D05916ED4B6BB NewGridCoord_YIndex_4_0534BDCC457A222D875D05916ED4B6BB)))
    (`|ExecutionSequence`
      (:`then_0`
        (bind (_foundplayerunit _playerunitarrayindex _result_found) (`self.GetPlayerUnitByGridCoord` OwningPlayerSlotIndex (`local.OriginGridCoord`) _playerunits))
        (if _result_found
          (bind _structout (setmembers `/Game/03_GameplayAssets/04_Data/01_Structs/ST_PlayerUnit` :`StructRef` _foundplayerunit :`GridX` _newgridcoord_xindex_2 :`GridY` _newgridcoord_yindex_2))
          (`KismetArrayLibrary.Array_Set` (`self.PlayerUnits`) _playerunitarrayindex _structout)
          (else
            (`KismetArrayLibrary.Array_Add` _playerunits (make `/Game/03_GameplayAssets/04_Data/01_Structs/ST_PlayerUnit` (`local.OwningPlayerSlotIndex`) _newgridcoord_xindex _newgridcoord_yindex (`local.UnitTypeRowName`) (`local.UnitStats_RowName`)))))))))

(fn `Upgrade Player Unit`
  (params (OwningPlayerSlotIndex :type Integer) (GridPos :type "/Game/03_GameplayAssets/04_Data/01_Structs/ST_GridCoords Structure") (NewUnitStatsRowName :type Name))
  (bind (_foundplayerunit _playerunitarrayindex _result_found) (`self.GetPlayerUnitByGridCoord` OwningPlayerSlotIndex GridPos (`self.PlayerUnits`)))
  (if _result_found
    (bind _structout (setmembers `/Game/03_GameplayAssets/04_Data/01_Structs/ST_PlayerUnit` :`StructRef` _foundplayerunit :`UnitStats_RowName` NewUnitStatsRowName))
    (`KismetArrayLibrary.Array_Set` (`self.PlayerUnits`) _playerunitarrayindex _structout)))

(fn `UserConstructionScript`
  (`parent.UserConstructionScript`)
  (if (`KismetSystemLibrary.IsServer`)
    (set `self.IngamePlayerData` (`/Game/03_GameplayAssets/06_GameSystem/01_GameInstances/BP_AMB_GameInstance.IngamePlayerData` (`/Game/03_GameplayAssets/01_Blueprints/90_MacroLibs/BPFL_GetGameSystem.GetAMBGameInstance`)))))