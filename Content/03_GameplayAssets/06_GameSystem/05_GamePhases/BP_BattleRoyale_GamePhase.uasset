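; Game phase that runs the Battle Royale round on the BattleRoyaleIsland, delegating setup, combat and cleanup to it through phase events.
; It fields earlier island winners' armies, or shuffled armies of all alive players when two or fewer remain.
; The island's outcome ends the phase early, while a timeout forces the battle to finish.
; Final results add first-battle kill scores and give losers damage before reaching the GameState.
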(event `self.PreparatePhase`
  (`parent.PreparatePhase`)
  (set `self.IsBattleRoyaleFinished` false)
  (`self.AssignPlayersToBattle`))

(event `self.ActivePhase`
  (`parent.ActivePhase`)
  (`self.ActivateBattleCombat`))

(event `self.DepreparatePhase`
  (`parent.DepreparatePhase`)
  (`self.DeactivateBattleCombat`)
  (if (`self.IsBattleRoyaleFinished`)
    (`self.FinalizeDepreparation`)
    (else
      (set `self.IsTimedOut` true)
      (`/Game/03_GameplayAssets/01_Blueprints/01_Actors/03_Grid/BP_BattleRoyaleIsland.BattleFinished` (`/Game/03_GameplayAssets/06_GameSystem/02_GameModes/BP_AutoBattlerIngameMode.BattleRoyaleIsland` (`self.GameModeContext`))))))

(event `self.TransitionNextPhase`
  (`parent.TransitionNextPhase`)
  (`self.CleanUpBattleRoyaleIsland`))

(fn `ActivateBattleCombat`
  (`/Game/03_GameplayAssets/01_Blueprints/01_Actors/03_Grid/BP_BattleRoyaleIsland.StartBattleUnitsCombat` (`/Game/03_GameplayAssets/06_GameSystem/02_GameModes/BP_AutoBattlerIngameMode.BattleRoyaleIsland` (`self.GameModeContext`))))

(fn `AssignPlayersToBattle`
  (locals (BattleRoyalePlayers :type "Array of /Game/03_GameplayAssets/04_Data/01_Structs/ST_BattleRoyalePlayerArmy Structure"))
  (bind _battleroyaleisland (`/Game/03_GameplayAssets/06_GameSystem/02_GameModes/BP_AutoBattlerIngameMode.BattleRoyaleIsland` (`self.GameModeContext`)))
  (bind _playerunitsarray (`self.GetPlayersUnitArray`))
  (for (_array_element _array_index) _playerunitsarray
    (bind _playerunits (break `/Game/03_GameplayAssets/04_Data/01_Structs/ST_Player_Unit_Array` _array_element))
    (`KismetArrayLibrary.Array_Add` (`local.BattleRoyalePlayers`) (make `/Game/03_GameplayAssets/04_Data/01_Structs/ST_BattleRoyalePlayerArmy` :`PlayerSlotIndex` (`.OwningPlayerSlotIndex_12_8369573341323E2A295DAEA2ED3DA911` (break `/Game/03_GameplayAssets/04_Data/01_Structs/ST_PlayerUnit` (`|GetArrayItem` _playerunits))) :`PlayerArmyStruct` _playerunits :`RemainingPlayerUnitCount` (`KismetArrayLibrary.Array_Length` _playerunits))))
  (`/Game/03_GameplayAssets/01_Blueprints/01_Actors/03_Grid/BP_BattleRoyaleIsland.AssignPlayerArmiesToFields` _battleroyaleisland (`local.BattleRoyalePlayers`))
  (add `/Game/03_GameplayAssets/01_Blueprints/01_Actors/03_Grid/BP_BattleRoyaleIsland.BattleRoyaleOutcome` _battleroyaleisland (`|CreateDelegate` :!event `OnBattleRoyaleRecievedOutcome`))
  (`/Game/03_GameplayAssets/01_Blueprints/01_Actors/03_Grid/BP_BattleRoyaleIsland.PrepareBattle` _battleroyaleisland))

(fn `CleanUpBattleRoyaleIsland`
  (`/Game/03_GameplayAssets/01_Blueprints/01_Actors/03_Grid/BP_BattleRoyaleIsland.CleanUpBattle` (`/Game/03_GameplayAssets/06_GameSystem/02_GameModes/BP_AutoBattlerIngameMode.BattleRoyaleIsland` (`self.GameModeContext`))))

(fn `DeactivateBattleCombat`
  (`/Game/03_GameplayAssets/01_Blueprints/01_Actors/03_Grid/BP_BattleRoyaleIsland.StopBattleUnitsCombat` (`/Game/03_GameplayAssets/06_GameSystem/02_GameModes/BP_AutoBattlerIngameMode.BattleRoyaleIsland` (`self.GameModeContext`))))

(fn `FinalizeDepreparation`
  (`self.SendLoosersNotifications`))

(fn `GetPlayersUnitArray`
  (returns (PlayerUnitsArray :type "Array of /Game/03_GameplayAssets/04_Data/01_Structs/ST_Player_Unit_Array Structure"))
  (locals (PUnitsArray :type "Array of /Game/03_GameplayAssets/04_Data/01_Structs/ST_Player_Unit_Array Structure") (AlivePSlotInidices :type "Array of Integer"))
  (bind _gamestatecontext (`self.GameStateContext`))
  (if (<= (`/Game/03_GameplayAssets/06_GameSystem/03_GameStates/BP_AMB_IngameState.GetCountAlivePlayerSlotindices` _gamestatecontext) 2)
    (`KismetArrayLibrary.Array_Clear` (`local.PUnitsArray`))
    (bind _output_get (set `local.AlivePSlotInidices` (`/Game/03_GameplayAssets/06_GameSystem/03_GameStates/BP_AMB_IngameState.AlivePlayerSlotIndices` _gamestatecontext)))
    (`KismetArrayLibrary.Array_Shuffle` _output_get)
    (for _array_element (`local.AlivePSlotInidices`)
      (bind _outplayerowningunits (`/Game/03_GameplayAssets/06_GameSystem/03_GameStates/BP_AMB_IngameState.GetPlayerUnitsOfPlayerSlotIndex` (`self.GameStateContext`) _array_element))
      (`KismetArrayLibrary.Array_Add` (`local.PUnitsArray`) (make `/Game/03_GameplayAssets/04_Data/01_Structs/ST_Player_Unit_Array` _outplayerowningunits)))
    (return (`local.PUnitsArray`))
    (else
      (return (`/Game/03_GameplayAssets/06_GameSystem/03_GameStates/BP_AMB_IngameState.WinningPlayerUnitsByBattleIsland` (`self.GameStateContext`))))))

(fn `OnBattleRoyaleRecievedOutcome`
  (params (PlayerBattleResults :type "Array of /Game/03_GameplayAssets/04_Data/01_Structs/ST_BattleResult Structure (by ref)"))
  (set `self.Player Battle Results` PlayerBattleResults)
  (if (not (`self.IsBattleRoyaleFinished`))
    (set `self.IsBattleRoyaleFinished` true)
    (if (`self.IsTimedOut`)
      (`self.FinalizeDepreparation`)
      (else
        (`/Game/03_GameplayAssets/06_GameSystem/02_GameModes/BP_AutoBattlerIngameMode.EnterNextStateCurrentGamePhase` (`self.GameModeContext`))))))

(fn `SendLoosersNotifications`
  (locals (`Aggregate Result` :type "/Game/03_GameplayAssets/04_Data/01_Structs/ST_BattleResult Structure") (BattleRoyaleLostDamage :type Integer :default 1))
  (for (_array_element _array_index) (`self.Player Battle Results`)
    (bind _output_get (set `local.Aggregate Result` _array_element))
    (for _array_element_2 (`/Game/03_GameplayAssets/06_GameSystem/03_GameStates/BP_AMB_IngameState.BattleOneResults` (`self.GameStateContext`))
      (bind ((`KillScore_15_0652BE904981294D1B69E6A9E9BF2B9D` _killscore) (`SlotID_26_92C8071B4C405CF822BF6F870D5CE8AE` _slotid)) (break `/Game/03_GameplayAssets/04_Data/01_Structs/ST_BattleResult` _array_element_2))
      (bind (_winner _killscore_2 _remainingunits _losthealth _unitskilled _slotid_2) (break `/Game/03_GameplayAssets/04_Data/01_Structs/ST_BattleResult` _output_get))
      (if (== _slotid _slotid_2)
        (set `local.Aggregate Result` (make `/Game/03_GameplayAssets/04_Data/01_Structs/ST_BattleResult` _winner (+ _killscore_2 _killscore) _remainingunits (`KismetMathLibrary.SelectInt` 0 (`local.BattleRoyaleLostDamage`) _winner) _unitskilled _slotid))
        (break)))
    (`/Game/03_GameplayAssets/06_GameSystem/03_GameStates/BP_AMB_IngameState.RecieveOutcome` (`self.GameStateContext`) (`local.Aggregate Result`)))
  (`KismetArrayLibrary.Array_Clear` (`/Game/03_GameplayAssets/06_GameSystem/03_GameStates/BP_AMB_IngameState.BattleOneResults` (`self.GameStateContext`))))