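; Base game phase Blueprint that runs a phase through preparation, active and depreparation states before handing off to the next phase.
; InitGamePhase caches the game mode, game instance and game state contexts.
; Each state event reads its duration from the DT_GamePhases row named by the settings handle and starts the game mode's phase timer.
; TransitionNextPhase fires the OnTriggerNextPhase dispatcher to signal the handoff.
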(event `PreparatePhase`
  (`self.TriggerGamePhaseStateTimer` "NewEnumerator0"))

(event `ActivePhase`
  (`self.TriggerGamePhaseStateTimer` "NewEnumerator1"))

(event `DepreparatePhase`
  (`self.TriggerGamePhaseStateTimer` "NewEnumerator2"))

(event `TransitionNextPhase`
  (`self.OnTriggerNextPhase`))

(fn `InitGamePhase`
  (params (GameModeContext :type "/Game/03_GameplayAssets/06_GameSystem/02_GameModes/BP_AutoBattlerIngameMode Object Reference") (GameInstanceContext :type "/Game/03_GameplayAssets/06_GameSystem/01_GameInstances/BP_AMB_GameInstance Object Reference") (GameStateContext :type "/Game/03_GameplayAssets/06_GameSystem/03_GameStates/BP_AMB_IngameState Object Reference"))
  (set `self.GameModeContext` GameModeContext)
  (set `self.GameInstanceContext` GameInstanceContext)
  (set `self.GameStateContext` GameStateContext))

(fn `TriggerGamePhaseStateTimer`
  (params (GamePhaseState :type "/Game/03_GameplayAssets/04_Data/02_Enums/E_GamePhase_States Enum" :default "NewEnumerator0"))
  (bind (_gamephasesettingshandle_datatable _gamephasesettingshandle_rowname) (break `DataTableRowHandle` (`self.GamePhaseSettingsHandle`)))
  (bind _returnvalue (`|GetDataTableRow` "/Game/03_GameplayAssets/04_Data/03_DataTables/DT_GamePhases.DT_GamePhases" _gamephasesettingshandle_rowname)
    (:`then`
      (switch `/Game/03_GameplayAssets/04_Data/02_Enums/E_GamePhase_States` GamePhaseState
        (:`NewEnumerator0`
          (bind (_phasesettings_preparationtime _phasesettings_activetime _phasesettings_depreparationtime) (break `/Game/03_GameplayAssets/04_Data/01_Structs/ST_GamePhaseSettings` (break `/Game/03_GameplayAssets/04_Data/01_Structs/ST_GamePhase` _returnvalue)))
          (`/Game/03_GameplayAssets/06_GameSystem/02_GameModes/BP_AutoBattlerIngameMode.StartGamePhaseTimer` (`self.GameModeContext`) _phasesettings_preparationtime))
        (:`NewEnumerator1`
          (`/Game/03_GameplayAssets/06_GameSystem/02_GameModes/BP_AutoBattlerIngameMode.StartGamePhaseTimer` (`self.GameModeContext`) _phasesettings_activetime))
        (:`NewEnumerator2`
          (`/Game/03_GameplayAssets/06_GameSystem/02_GameModes/BP_AutoBattlerIngameMode.StartGamePhaseTimer` (`self.GameModeContext`) _phasesettings_depreparationtime))))))