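; Game phase for the first battle round, pairing alive players randomly on battle islands and running their army combat.
; With an odd player count, slot 8 fights as a clone of a random player's army.
; Island outcomes are collected until all active islands report, advancing the phase early; on timeout, deprepare triggers match evaluation.
; Finalizing stores winners' surviving units and passes results to the game state, and transition cleans up the islands.
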(event `self.PreparatePhase`
  (`parent.PreparatePhase`)
  (set `self.IsBattleOneFinished` false)
  (set `self.IsTimedOut` false)
  (`KismetArrayLibrary.Array_Clear` (`self.BattleOutcomes`))
  (`KismetArrayLibrary.Array_Clear` (`self.Results`))
  (`self.AssignPlayerToBattles` (`/Game/03_GameplayAssets/06_GameSystem/03_GameStates/BP_AMB_IngameState.AlivePlayerSlotIndices` (`self.GameStateContext`))))

(event `self.ActivePhase`
  (`parent.ActivePhase`)
  (`self.ActivateBattleCombat`))

(event `self.DepreparatePhase`
  (`parent.DepreparatePhase`)
  (`self.DeactivateBattleCombat`)
  (if (`self.IsBattleOneFinished`)
    (`self.FinalizeDepreparation`)
    (else
      (set `self.IsTimedOut` true)
      (`self.EvaluateBattles`))))

(event `self.TransitionNextPhase`
  (`parent.TransitionNextPhase`)
  (for _array_element (`/Game/03_GameplayAssets/06_GameSystem/02_GameModes/BP_AutoBattlerIngameMode.BattleIslands` (`self.GameModeContext`))
    (`/Game/03_GameplayAssets/01_Blueprints/01_Actors/03_Grid/BP_BattleOneIsland.CleanUpBattle` _array_element)))

(event `RecievedIslandOutcome`
  (params (IslandOutcome :type "/Game/03_GameplayAssets/04_Data/01_Structs/ST_BattleOutcome Structure") (PlayerAResult :type "/Game/03_GameplayAssets/04_Data/01_Structs/ST_BattleResult Structure") (PlayerBResult :type "/Game/03_GameplayAssets/04_Data/01_Structs/ST_BattleResult Structure"))
  (bind _results (`self.Results`))
  (if (not (`self.IsBattleOneFinished`))
    (`KismetArrayLibrary.Array_Add` (`self.BattleOutcomes`) IslandOutcome)
    (`KismetArrayLibrary.Array_Add` _results PlayerAResult)
    (`KismetArrayLibrary.Array_Add` _results PlayerBResult)
    (if (== (`/Game/03_GameplayAssets/06_GameSystem/03_GameStates/BP_AMB_IngameState.ActiveBattleIslands` (`self.GameStateContext`)) (`KismetArrayLibrary.Array_Length` (`self.BattleOutcomes`)))
      (set `self.IsBattleOneFinished` true)
      (if (`self.IsTimedOut`)
        (`self.FinalizeDepreparation`)
        (else
          (`/Game/03_GameplayAssets/06_GameSystem/02_GameModes/BP_AutoBattlerIngameMode.EnterNextStateCurrentGamePhase` (`self.GameModeContext`)))))))

(fn `ActivateBattleCombat`
  (for _array_element (`/Game/03_GameplayAssets/06_GameSystem/02_GameModes/BP_AutoBattlerIngameMode.BattleIslands` (`self.GameModeContext`))
    (`/Game/03_GameplayAssets/01_Blueprints/01_Actors/03_Grid/BP_BattleOneIsland.StartBattleUnitsCombat` _array_element)))

(fn `AssignPlayerToBattles`
  (params (AlivePlayersSlotIndex :type "Array of Integer"))
  (returns (SortedEnemySlotIDs :type "Array of Integer"))
  (locals (ShuffledAlivePlayersSlotIndex :type "Array of Integer") (IsCopy :type Boolean) (temp :type "Array of Integer") (tempArmy :type "Array of /Game/03_GameplayAssets/04_Data/01_Structs/ST_PlayerUnit Structure"))
  (bind _gamestatecontext (`self.GameStateContext`))
  (bind _gamestatecontext_2 (`self.GameStateContext`))
  (bind _playerunits (`/Game/03_GameplayAssets/06_GameSystem/03_GameStates/BP_AMB_IngameState.PlayerUnits` _gamestatecontext_2))
  (bind _returnvalue (!= (mod (`KismetArrayLibrary.Array_Length` AlivePlayersSlotIndex) 2) 0))
  (`|ExecutionSequence`
    (:`then_0`
      (set `/Game/03_GameplayAssets/06_GameSystem/03_GameStates/BP_AMB_IngameState.ActiveBattleIslands` 0 _gamestatecontext)
      (set `/Game/03_GameplayAssets/06_GameSystem/03_GameStates/BP_AMB_IngameState.ResolvedBattleIslands` 0 _gamestatecontext)
      (bind _output_get (set `local.ShuffledAlivePlayersSlotIndex` AlivePlayersSlotIndex))
      (`KismetArrayLibrary.Array_Shuffle` _output_get)
      (set `local.IsCopy` _returnvalue)
      (if _returnvalue
        ;[1 1 1] Add Player Slot 8 to index array
        (bind _outshuffledaliveplayersslotindex (`self.FillPlayersToEven` (`local.ShuffledAlivePlayersSlotIndex`)))
        (set `local.ShuffledAlivePlayersSlotIndex` _outshuffledaliveplayersslotindex))
      (for (_array_element _array_index) (`/Game/03_GameplayAssets/06_GameSystem/02_GameModes/BP_AutoBattlerIngameMode.BattleIslands` (`self.GameModeContext`))
        (add `/Game/03_GameplayAssets/01_Blueprints/01_Actors/03_Grid/BP_BattleOneIsland.BattleOutcome` _array_element (`|CreateDelegate` :!event `RecievedIslandOutcome`))
        (bind _returnvalue_2 (* _array_index 2))
        (if (< _returnvalue_2 (`KismetArrayLibrary.Array_Length` (`local.ShuffledAlivePlayersSlotIndex`)))
          (`|ExecutionSequence`
            (:`then_0`
              (bind _output (`|GetArrayItem` (`local.ShuffledAlivePlayersSlotIndex`) _returnvalue_2))
              (bind _outplayerowningunits (`/Game/03_GameplayAssets/06_GameSystem/03_GameStates/BP_AMB_IngameState.GetPlayerUnitsOfPlayerSlotIndex` (`self.GameStateContext`) _output))
              (set `/Game/03_GameplayAssets/01_Blueprints/01_Actors/03_Grid/BP_BattleOneIsland.PlayerArmyA` _outplayerowningunits _array_element)
              (set `/Game/03_GameplayAssets/01_Blueprints/01_Actors/03_Grid/BP_BattleOneIsland.PlayerASlotIndex` _output _array_element))
            (:`then_1`
              (bind _output_2 (`|GetArrayItem` (`local.ShuffledAlivePlayersSlotIndex`) (+ _returnvalue_2 1)))
              (if (== 8 _output_2)
                (bind _output_get_2 (set `local.temp` (`local.ShuffledAlivePlayersSlotIndex`)))
                (`KismetArrayLibrary.Array_RemoveItem` _output_get_2 8)
                (bind _outplayerowningunits_2 (`/Game/03_GameplayAssets/06_GameSystem/03_GameStates/BP_AMB_IngameState.GetPlayerUnitsOfPlayerSlotIndex` _gamestatecontext_2 (`KismetArrayLibrary.Array_Random` (`local.temp`))))
                (bind _output_get_3 (set `/Game/03_GameplayAssets/01_Blueprints/01_Actors/03_Grid/BP_BattleOneIsland.PlayerArmyB` _outplayerowningunits_2 _array_element))
                (set `/Game/03_GameplayAssets/01_Blueprints/01_Actors/03_Grid/BP_BattleOneIsland.PlayerBSlotIndex` 8 _array_element)
                (bind _outplayerowningunits_3 (`/Game/03_GameplayAssets/06_GameSystem/03_GameStates/BP_AMB_IngameState.GetPlayerUnitsOfPlayerSlotIndex` _gamestatecontext_2 8))
                (for _array_element_2 _outplayerowningunits_3
                  (`KismetArrayLibrary.Array_RemoveItem` _playerunits _array_element_2))
                (for _array_element_3 _output_get_3
                  (bind _structout (setmembers `/Game/03_GameplayAssets/04_Data/01_Structs/ST_PlayerUnit` :`StructRef` _array_element_3 :`OwningPlayerSlotIndex` 8))
                  (`KismetArrayLibrary.Array_Append` _playerunits (`|MakeArray` _structout)))
                (else
                  (bind _outplayerowningunits_4 (`/Game/03_GameplayAssets/06_GameSystem/03_GameStates/BP_AMB_IngameState.GetPlayerUnitsOfPlayerSlotIndex` _gamestatecontext_2 _output_2))
                  (set `/Game/03_GameplayAssets/01_Blueprints/01_Actors/03_Grid/BP_BattleOneIsland.PlayerArmyB` _outplayerowningunits_4 _array_element)
                  (bind _output_get_4 (set `/Game/03_GameplayAssets/01_Blueprints/01_Actors/03_Grid/BP_BattleOneIsland.PlayerBSlotIndex` _output_2 _array_element)))))
            (:`then_2`
              (`|ExecutionSequence`
                (:`then_0`
                  (bind (_playercontroller _success) (`/Game/03_GameplayAssets/06_GameSystem/03_GameStates/BP_AMB_IngameState.GetPlayerControllerBySlotIndex` (`self.GameStateContext`) _output))
                  (if _success
                    (bind _returnvalue_3 (/ (+ (`SceneComponent.K2_GetComponentLocation` (`/Game/03_GameplayAssets/01_Blueprints/01_Actors/03_Grid/BP_BattleOneIsland.BattleGridB` _array_element)) (`SceneComponent.K2_GetComponentLocation` (`/Game/03_GameplayAssets/01_Blueprints/01_Actors/03_Grid/BP_BattleOneIsland.BattleGridA` _array_element))) 2))
                    (`/Game/03_GameplayAssets/01_Blueprints/01_Actors/01_Player/BP_AutoBattlerIngameController.ClientTeleportToBattleOne` _playercontroller _returnvalue_3)))
                (:`then_1`
                  (bind (_playercontroller_2 _success_2) (`/Game/03_GameplayAssets/06_GameSystem/03_GameStates/BP_AMB_IngameState.GetPlayerControllerBySlotIndex` (`self.GameStateContext`) _output_2))
                  (if _success_2
                    (`/Game/03_GameplayAssets/01_Blueprints/01_Actors/01_Player/BP_AutoBattlerIngameController.ClientTeleportToBattleOne` _playercontroller_2 _returnvalue_3)))
                (:`then_2`
                  (if (== _output_get_4 8)
                    (bind (_playeridentifier _playername) (break `/Game/03_GameplayAssets/04_Data/01_Structs/ST_PlayerData` (`/Game/03_GameplayAssets/01_Blueprints/01_Actors/01_Player/BP_AutoBattlerIngameController.OwnPlayerData` _playercontroller)))
                    (`/Game/03_GameplayAssets/01_Blueprints/01_Actors/01_Player/BP_AutoBattlerIngameController.Client_DisplayMessage` _playercontroller (`|FormatText` "{PA} vs. A Cloned Army" _playername))
                    (else
                      (bind _result (`|FormatText` "{PA} vs. {PB}" _playername (`.PlayerName_3_C95595434AD221FD6BC8A0AA4493A191` (break `/Game/03_GameplayAssets/04_Data/01_Structs/ST_PlayerData` (`/Game/03_GameplayAssets/01_Blueprints/01_Actors/01_Player/BP_AutoBattlerIngameController.OwnPlayerData` _playercontroller_2)))))
                      (`/Game/03_GameplayAssets/01_Blueprints/01_Actors/01_Player/BP_AutoBattlerIngameController.Client_DisplayMessage` _playercontroller _result)
                      (`/Game/03_GameplayAssets/01_Blueprints/01_Actors/01_Player/BP_AutoBattlerIngameController.Client_DisplayMessage` _playercontroller_2 _result))))))
            (:`then_3`
              (`/Game/03_GameplayAssets/01_Blueprints/01_Actors/03_Grid/BP_BattleOneIsland.PrepareBattle` _array_element)
              (`/Engine/EditorBlueprintResources/StandardMacros.IncrementInt` (`/Game/03_GameplayAssets/06_GameSystem/03_GameStates/BP_AMB_IngameState.ActiveBattleIslands` (`self.GameStateContext`)))))
          (else
            (break)))))
    (:`then_1`
      (return (`local.ShuffledAlivePlayersSlotIndex`)))))

(fn `DeactivateBattleCombat`
  (for _array_element (`/Game/03_GameplayAssets/06_GameSystem/02_GameModes/BP_AutoBattlerIngameMode.BattleIslands` (`self.GameModeContext`))
    (`/Game/03_GameplayAssets/01_Blueprints/01_Actors/03_Grid/BP_BattleOneIsland.StopBattleUnitsCombat` _array_element)))

(fn `EvaluateBattles`
  (for _array_element (`/Game/03_GameplayAssets/06_GameSystem/02_GameModes/BP_AutoBattlerIngameMode.BattleIslands` (`self.GameModeContext`))
    (if (> (`KismetArrayLibrary.Array_Length` (`/Game/03_GameplayAssets/01_Blueprints/01_Actors/03_Grid/BP_BattleOneIsland.PlayerArmyA` _array_element)) 0)
      (if (`/Game/03_GameplayAssets/01_Blueprints/01_Actors/03_Grid/BP_BattleOneIsland.Evaluated` _array_element)
        (`/Game/03_GameplayAssets/01_Blueprints/01_Actors/03_Grid/BP_BattleOneIsland.EvaluateMatch` _array_element)))))

(fn `FillPlayersToEven`
  (params (ShuffledAlivePlayersSlotIndex :type "Array of Integer"))
  (returns (OutShuffledAlivePlayersSlotIndex :type "Array of Integer"))
  (`KismetArrayLibrary.Array_Add` ShuffledAlivePlayersSlotIndex 8)
  (return ShuffledAlivePlayersSlotIndex))

(fn `FinalizeDepreparation`
  (`self.ResolveWiningPlayerRemainingUnits`)
  (`self.SendLoosersNotifications`))

(fn `ResolveWiningPlayerRemainingUnits`
  (`KismetArrayLibrary.Array_Clear` (`/Game/03_GameplayAssets/06_GameSystem/03_GameStates/BP_AMB_IngameState.WinningPlayerUnitsByBattleIsland` (`self.GameStateContext`)))
  (for _array_element (`/Game/03_GameplayAssets/06_GameSystem/02_GameModes/BP_AutoBattlerIngameMode.BattleIslands` (`self.GameModeContext`))
    (bind _playeraslotindex (`/Game/03_GameplayAssets/01_Blueprints/01_Actors/03_Grid/BP_BattleOneIsland.PlayerASlotIndex` _array_element))
    (if (and (< _playeraslotindex 8) (>= _playeraslotindex 0))
      (bind (_winingplayerremainingunits _winningplayerslotindex) (`/Game/03_GameplayAssets/01_Blueprints/01_Actors/03_Grid/BP_BattleOneIsland.GetWinningPlayerRemainingUnits` _array_element))
      (if (< _winningplayerslotindex 8)
        (`KismetArrayLibrary.Array_Add` (`/Game/03_GameplayAssets/06_GameSystem/03_GameStates/BP_AMB_IngameState.WinningPlayerUnitsByBattleIsland` (`self.GameStateContext`)) (make `/Game/03_GameplayAssets/04_Data/01_Structs/ST_Player_Unit_Array` _winingplayerremainingunits))))))

(fn `SendLoosersNotifications`
  (bind _gamestatecontext (`self.GameStateContext`))
  (for (_array_element _array_index) (`self.Results`)
    (if (`.Winner_12_0340D3404E91CB2A5ABBB791F05AE15D` (break `/Game/03_GameplayAssets/04_Data/01_Structs/ST_BattleResult` _array_element))
      (`/Game/03_GameplayAssets/06_GameSystem/03_GameStates/BP_AMB_IngameState.RecieveBattleOneResult` _gamestatecontext _array_element)
      (else
        (`/Game/03_GameplayAssets/06_GameSystem/03_GameStates/BP_AMB_IngameState.RecieveOutcome` _gamestatecontext _array_element)))))