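; Behavior tree task that orders the AI-controlled unit to attack the unit stored in the CurrentTarget blackboard key.
; It casts both the target and the controlled pawn to BP_Unit, then calls AttackTarget if their distance is within the attacker's Range stat.
; The task succeeds once the attack is issued, and fails when out of range or when a cast fails, printing a debug message for failed casts.
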(event `self.ReceiveExecuteAI`
  (params (OwnerController :type "AIController Object Reference") (ControlledPawn :type "Pawn Object Reference"))
  (bind _returnvalue (`BTFunctionLibrary.GetBlackboardValueAsActor` (`self.CurrentTarget`)))
  (bind _asbp_unit (cast `/Game/03_GameplayAssets/01_Blueprints/01_Actors/02_Unit/BP_Unit` _returnvalue)
    (:`then`
      (bind _asbp_unit_2 (cast `/Game/03_GameplayAssets/01_Blueprints/01_Actors/02_Unit/BP_Unit` ControlledPawn)
        (:`then`
          (if (<= (`Actor.GetDistanceTo` _asbp_unit _asbp_unit_2) (`.Range_5_F1A0ADFA410819004523D4B1276AD43D` (break `/Game/03_GameplayAssets/04_Data/01_Structs/ST_Unit_Stats` (`/Game/03_GameplayAssets/01_Blueprints/01_Actors/02_Unit/BP_Unit.Stats` _asbp_unit_2))))
            (`/Game/03_GameplayAssets/01_Blueprints/01_Actors/02_Unit/BP_Unit.AttackTarget` _asbp_unit_2 _asbp_unit)
            (`self.FinishExecute` true)
            (else
              (`self.FinishExecute` false))))
        (:`CastFailed`
          (`KismetSystemLibrary.PrintText` (`|FormatText` "{obj} did not Cast to Unit" ControlledPawn))
          (`self.FinishExecute` false))))
    (:`CastFailed`
      (`KismetSystemLibrary.PrintText` (`|FormatText` "{obj} did not Cast to Unit" _returnvalue))
      (`self.FinishExecute` false))))