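; Behavior tree task that picks the closest target for an AI controlled by 99_BP_NewAI.
; It finds the TargetList actor nearest the pawn's nav agent location and writes it to the SetTarget blackboard key.
; An empty list stops the brain component's logic but still finishes successfully, while a failed controller cast prints a message and fails the task.
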(event `self.ReceiveExecuteAI`
  (params (OwnerController :type "AIController Object Reference") (ControlledPawn :type "Pawn Object Reference"))
  (bind _as99_bp_new_ai (cast `/Game/99_Testing_Max/05_AI/AIv2/99_BP_NewAI` OwnerController)
    (:`then`
      (bind _targetlist (`/Game/99_Testing_Max/05_AI/AIv2/99_BP_NewAI.TargetList` _as99_bp_new_ai))
      (if (!= (`KismetArrayLibrary.Array_Length` _targetlist) 0)
        (`BTFunctionLibrary.SetBlackboardValueAsObject` (`self.SetTarget`) (`.ReturnValue` (`GameplayStatics.FindNearestActor` (`Pawn.GetNavAgentLocation` ControlledPawn) _targetlist)))
        (`self.FinishExecute` true)
        (else
          (`BrainComponent.StopLogic` (`AIController.BrainComponent` _as99_bp_new_ai) "")
          (`self.FinishExecute` true))))
    (:`CastFailed`
      (`KismetSystemLibrary.PrintText` (`|FormatText` "{obj} did not Cast to NewAI" OwnerController))
      (`self.FinishExecute` false))))