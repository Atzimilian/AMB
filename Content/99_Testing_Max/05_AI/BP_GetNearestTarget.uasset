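; Behavior Tree task that picks a BP_Unit as the nearest target to the controlled pawn and writes it to the BBTarget Blackboard key.
; It searches only when CurrentClosest is unset or equals the pawn, using the pawn as a placeholder while comparing distances.
; The pawn is not filtered from the actor list, and an already cached target skips the search.
; The task finishes with success.
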(event `self.ReceiveExecuteAI`
  (params (OwnerController :type "AIController Object Reference") (ControlledPawn :type "Pawn Object Reference"))
  (bind _currentclosest (`self.CurrentClosest`))
  (bind _returnvalue (== _currentclosest ControlledPawn))
  (if _returnvalue
    (bind _outactors (`GameplayStatics.GetAllActorsOfClass` "/Game/03_GameplayAssets/01_Blueprints/01_Actors/02_Unit/BP_Unit.BP_Unit_C" :!label _label))
    (for _array_element _outactors
      (if _returnvalue
        (bind _output_get (set `self.CurrentClosest` _array_element :!label _label_2))
        (elif (< (`Actor.GetDistanceTo` _array_element ControlledPawn) (`Actor.GetDistanceTo` (`self.CurrentClosest`) ControlledPawn))
          (goto _label_2))))
    (`BTFunctionLibrary.SetBlackboardValueAsObject` (`self.BB_Target`) _output_get)
    (elif (!= _currentclosest null)
      _
      (else
        (set `self.CurrentClosest` ControlledPawn)
        (goto _label))))
  (`self.FinishExecute` true))